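; BP_MovingWheel is an actor with a spinning gear mesh that slides back and forth along the Y axis.
; A RotatingMovement component targets the StylizedGear at BeginPlay to handle the spin.
; Tick offsets the root's relative Y by Speed scaled by delta time, negating Speed whenever the absolute Y exceeds a fixed limit.
; That limit is measured from zero in the root's relative space, rather than from the starting position.
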(event `self.ReceiveBeginPlay`
  (`MovementComponent.SetUpdatedComponent` (`self.RotatingMovement`) (`self.StylizedGear`)))

(event `self.ReceiveTick`
  (params (DeltaSeconds :type "Float (single-precision)"))
  (bind (_relativelocation_x _relativelocation_y _relativelocation_z) (`KismetMathLibrary.BreakVector` (`SceneComponent.RelativeLocation` (`self.DefaultSceneRoot`))))
  (`SceneComponent.K2_SetRelativeLocation` (`self.DefaultSceneRoot`) (`KismetMathLibrary.MakeVector` _relativelocation_x (+ (* DeltaSeconds (`self.Speed`)) _relativelocation_y) _relativelocation_z) false false)
  (if (> (`KismetMathLibrary.Abs` _relativelocation_y) 195.0)
    (set `self.Speed` (* (`self.Speed`) -1.0))))

(fn `UserConstructionScript`)