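; BP_TableCover flips two rows of table cover panels in a domino sequence once BP_TablePuzzle is complete.
; Tick polls the puzzle, then a DoOnce and short delay start parallel left and right chains of per-panel timelines, each Finished starting the next.
; FlipMove rotates each panel in opposite directions per side, while FlipMatChange lights it yellow (left) or blue (right).
; The last right panel sets FlipComplete on BP_RearTableSwitch.
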(event `self.ReceiveBeginPlay`
  (bind _outactors (`GameplayStatics.GetAllActorsOfClass` "/Game/BoxesLike/BluePrints/Box2-2/BP_TablePuzzle.BP_TablePuzzle_C"))
  (set `self.TablePuzzle` (`|GetArrayItem` _outactors))
  (bind _outactors_2 (`GameplayStatics.GetAllActorsOfClass` "/Game/BoxesLike/BluePrints/Box2-2/BP_RearTableSwitch.BP_RearTableSwitch_C"))
  (set `self.RearTableSwitch` (`|GetArrayItem` _outactors_2)))

(event `self.ReceiveTick`
  (params (DeltaSeconds :type "Float (single-precision)"))
  (bind _sm_overturnpanell1 (`self.SM_OverTurnPanelL1`))
  (bind _sm_overturnpanell2 (`self.SM_OverTurnPanelL2`))
  (bind _sm_overturnpanell3 (`self.SM_OverTurnPanelL3`))
  (bind _sm_overturnpanell4 (`self.SM_OverTurnPanelL4`))
  (bind _sm_overturnpanell5 (`self.SM_OverTurnPanelL5`))
  (bind _sm_overturnpanelrstart (`self.SM_OverTurnPanelRStart`))
  (bind _sm_overturnpanell6 (`self.SM_OverTurnPanelL6`))
  (bind _sm_overturnpanell7 (`self.SM_OverTurnPanelL7`))
  (bind _sm_overturnpanell8 (`self.SM_OverTurnPanelL8`))
  (bind _sm_overturnpanell9 (`self.SM_OverTurnPanelL9`))
  (bind _sm_overturnpanell10 (`self.SM_OverTurnPanelL10`))
  (bind _sm_overturnpanell11 (`self.SM_OverTurnPanelL11`))
  (bind _sm_overturnpanell12 (`self.SM_OverTurnPanelL12`))
  (bind _sm_overturnpanellend (`self.SM_OverTurnPanelLEnd`))
  (bind _sm_overturnpanelr1 (`self.SM_OverTurnPanelR1`))
  (bind _sm_overturnpanelr2 (`self.SM_OverTurnPanelR2`))
  (bind _sm_overturnpanelr3 (`self.SM_OverTurnPanelR3`))
  (bind _sm_overturnpanelr4 (`self.SM_OverTurnPanelR4`))
  (bind _sm_overturnpanelr5 (`self.SM_OverTurnPanelR5`))
  (bind _sm_overturnpanelr6 (`self.SM_OverTurnPanelR6`))
  (bind _sm_overturnpanelr7 (`self.SM_OverTurnPanelR7`))
  (bind _sm_overturnpanelr8 (`self.SM_OverTurnPanelR8`))
  (bind _sm_overturnpanelr9 (`self.SM_OverTurnPanelR9`))
  (bind _sm_overturnpanelr10 (`self.SM_OverTurnPanelR10`))
  (bind _sm_overturnpanelr11 (`self.SM_OverTurnPanelR11`))
  (bind _sm_overturnpanelr12 (`self.SM_OverTurnPanelR12`))
  (bind _sm_overturnpanelrend (`self.SM_OverTurnPanelREnd`))
  (bind _sm_overturnpanellstart (`self.SM_OverTurnPanelLStart`))
  (if (`/Game/BoxesLike/BluePrints/Box2-2/BP_TablePuzzle.PuzzleComplete` (`self.TablePuzzle`))
    (`/Engine/EditorBlueprintResources/StandardMacros.DoOnce` false ; 판넬 회전 실시
      (:`Completed`
        (`KismetSystemLibrary.Delay` 2.0)
        (`|ExecutionSequence`
          (:`then_0`
            (bind (_direction _value) (`Timeline|LeftFlip`)
              (:`Update`
                (`self.FlipMove` _sm_overturnpanellstart _value 1.0))
              (:`Finished`
                (`self.FlipMatChange` _sm_overturnpanellstart true)
                (bind (_direction_2 _value_2) (`Timeline|Timeline`)
                  (:`Update`
                    (`self.FlipMove` _sm_overturnpanell1 _value_2 1.0))
                  (:`Finished`
                    (`self.FlipMatChange` _sm_overturnpanell1 true)
                    (bind (_direction_3 _value_3) (`Timeline|Timeline_0`)
                      (:`Update`
                        (`self.FlipMove` _sm_overturnpanell2 _value_3 1.0))
                      (:`Finished`
                        (`self.FlipMatChange` _sm_overturnpanell2 true)
                        (bind (_direction_4 _value_4) (`Timeline|Timeline_1`)
                          (:`Update`
                            (`self.FlipMove` _sm_overturnpanell3 _value_4 1.0))
                          (:`Finished`
                            (`self.FlipMatChange` _sm_overturnpanell3 true)
                            (bind (_direction_5 _value_5) (`Timeline|Timeline_2`)
                              (:`Update`
                                (`self.FlipMove` _sm_overturnpanell4 _value_5 1.0))
                              (:`Finished`
                                (`self.FlipMatChange` _sm_overturnpanell4 true)
                                (bind (_direction_6 _value_6) (`Timeline|Timeline_3`)
                                  (:`Update`
                                    (`self.FlipMove` _sm_overturnpanell5 _value_6 1.0))
                                  (:`Finished`
                                    (`self.FlipMatChange` _sm_overturnpanell5 true)
                                    (bind (_direction_7 _value_7) (`Timeline|Timeline_4`)
                                      (:`Update`
                                        (`self.FlipMove` _sm_overturnpanell6 _value_7 1.0))
                                      (:`Finished`
                                        (`self.FlipMatChange` _sm_overturnpanell6 true)
                                        (bind (_direction_8 _value_8) (`Timeline|Timeline_5`)
                                          (:`Update`
                                            (`self.FlipMove` _sm_overturnpanell7 _value_8 1.0))
                                          (:`Finished`
                                            (`self.FlipMatChange` _sm_overturnpanell7 true)
                                            (bind (_direction_9 _value_9) (`Timeline|Timeline_6`)
                                              (:`Update`
                                                (`self.FlipMove` _sm_overturnpanell8 _value_9 1.0))
                                              (:`Finished`
                                                (`self.FlipMatChange` _sm_overturnpanell8 true)
                                                (bind (_direction_10 _value_10) (`Timeline|Timeline_7`)
                                                  (:`Update`
                                                    (`self.FlipMove` _sm_overturnpanell9 _value_10 1.0))
                                                  (:`Finished`
                                                    (`self.FlipMatChange` _sm_overturnpanell9 true)
                                                    (bind (_direction_11 _value_11) (`Timeline|Timeline_8`)
                                                      (:`Update`
                                                        (`self.FlipMove` _sm_overturnpanell10 _value_11 1.0))
                                                      (:`Finished`
                                                        (`self.FlipMatChange` _sm_overturnpanell10 true)
                                                        (bind (_direction_12 _value_12) (`Timeline|Timeline_9`)
                                                          (:`Update`
                                                            (`self.FlipMove` _sm_overturnpanell11 _value_12 1.0))
                                                          (:`Finished`
                                                            (`self.FlipMatChange` _sm_overturnpanell11 true)
                                                            (bind (_direction_13 _value_13) (`Timeline|Timeline_10`)
                                                              (:`Update`
                                                                (`self.FlipMove` _sm_overturnpanell12 _value_13 1.0))
                                                              (:`Finished`
                                                                (`self.FlipMatChange` _sm_overturnpanell12 true)
                                                                (bind (_direction_14 _value_14) (`Timeline|Timeline_11`)
                                                                  (:`Update`
                                                                    (`self.FlipMove` _sm_overturnpanellend _value_14 1.0))
                                                                  (:`Finished`
                                                                    (`self.FlipMatChange` _sm_overturnpanellend true))))))))))))))))))))))))))))))
          (:`then_1`
            (bind (_direction_15 _value_15) (`Timeline|RightFlip`)
              (:`Update`
                (`self.FlipMove` _sm_overturnpanelrstart _value_15 -1.0))
              (:`Finished`
                (`self.FlipMatChange` _sm_overturnpanelrstart)
                (bind (_direction_16 _value_16) (`Timeline|Timeline_12`)
                  (:`Update`
                    (`self.FlipMove` _sm_overturnpanelr1 _value_16 -1.0))
                  (:`Finished`
                    (`self.FlipMatChange` _sm_overturnpanelr1)
                    (bind (_direction_17 _value_17) (`Timeline|Timeline_13`)
                      (:`Update`
                        (`self.FlipMove` _sm_overturnpanelr2 _value_17 -1.0))
                      (:`Finished`
                        (`self.FlipMatChange` _sm_overturnpanelr2)
                        (bind (_direction_18 _value_18) (`Timeline|Timeline_14`)
                          (:`Update`
                            (`self.FlipMove` _sm_overturnpanelr3 _value_18 -1.0))
                          (:`Finished`
                            (`self.FlipMatChange` _sm_overturnpanelr3)
                            (bind (_direction_19 _value_19) (`Timeline|Timeline_15`)
                              (:`Update`
                                (`self.FlipMove` _sm_overturnpanelr4 _value_19 -1.0))
                              (:`Finished`
                                (`self.FlipMatChange` _sm_overturnpanelr4)
                                (bind (_direction_20 _value_20) (`Timeline|Timeline_16`)
                                  (:`Update`
                                    (`self.FlipMove` _sm_overturnpanelr5 _value_20 -1.0))
                                  (:`Finished`
                                    (`self.FlipMatChange` _sm_overturnpanelr5)
                                    (bind (_direction_21 _value_21) (`Timeline|Timeline_17`)
                                      (:`Update`
                                        (`self.FlipMove` _sm_overturnpanelr6 _value_21 -1.0))
                                      (:`Finished`
                                        (`self.FlipMatChange` _sm_overturnpanelr6)
                                        (bind (_direction_22 _value_22) (`Timeline|Timeline_18`)
                                          (:`Update`
                                            (`self.FlipMove` _sm_overturnpanelr7 _value_22 -1.0))
                                          (:`Finished`
                                            (`self.FlipMatChange` _sm_overturnpanelr7)
                                            (bind (_direction_23 _value_23) (`Timeline|Timeline_19`)
                                              (:`Update`
                                                (`self.FlipMove` _sm_overturnpanelr8 _value_23 -1.0))
                                              (:`Finished`
                                                (`self.FlipMatChange` _sm_overturnpanelr8)
                                                (bind (_direction_24 _value_24) (`Timeline|Timeline_20`)
                                                  (:`Update`
                                                    (`self.FlipMove` _sm_overturnpanelr9 _value_24 -1.0))
                                                  (:`Finished`
                                                    (`self.FlipMatChange` _sm_overturnpanelr9)
                                                    (bind (_direction_25 _value_25) (`Timeline|Timeline_21`)
                                                      (:`Update`
                                                        (`self.FlipMove` _sm_overturnpanelr10 _value_25 -1.0))
                                                      (:`Finished`
                                                        (`self.FlipMatChange` _sm_overturnpanelr10)
                                                        (bind (_direction_26 _value_26) (`Timeline|Timeline_22`)
                                                          (:`Update`
                                                            (`self.FlipMove` _sm_overturnpanelr11 _value_26 -1.0))
                                                          (:`Finished`
                                                            (`self.FlipMatChange` _sm_overturnpanelr11)
                                                            (bind (_direction_27 _value_27) (`Timeline|Timeline_23`)
                                                              (:`Update`
                                                                (`self.FlipMove` _sm_overturnpanelr12 _value_27 -1.0))
                                                              (:`Finished`
                                                                (`self.FlipMatChange` _sm_overturnpanelr12)
                                                                (bind (_direction_28 _value_28) (`Timeline|Timeline_24`)
                                                                  (:`Update`
                                                                    (`self.FlipMove` _sm_overturnpanelrend _value_28 -1.0))
                                                                  (:`Finished`
                                                                    (`self.FlipMatChange` _sm_overturnpanelrend)
                                                                    (set `/Game/BoxesLike/BluePrints/Box2-2/BP_RearTableSwitch.FlipComplete` true (`self.RearTableSwitch`))))))))))))))))))))))))))))))))))))

(fn `FlipMatChange`
  (params (FlipPanel :type "StaticMeshComponent Object Reference") (LisTandRisF :type Boolean))
  (bind _staticmesh (`StaticMeshComponent.StaticMesh` (`local.FlipPanel`)))
  (bind _staticmesh_2 (`StaticMeshComponent.StaticMesh` (`local.FlipPanel`)))
  (bind _returnvalue (or (== _staticmesh "/Game/BoxesLike/StaticMesh/Box2-2/SM_FlipBoardBL.SM_FlipBoardBL") (== _staticmesh "/Game/BoxesLike/StaticMesh/Box2-2/SM_FlipBoardBR.SM_FlipBoardBR") (== _staticmesh "/Game/BoxesLike/StaticMesh/Box2-2/SM_FlipBoardTL.SM_FlipBoardTL") (== _staticmesh "/Game/BoxesLike/StaticMesh/Box2-2/SM_FlipBoardTR.SM_FlipBoardTR")))
  (bind _returnvalue_2 (or (== _staticmesh_2 "/Game/BoxesLike/StaticMesh/Box2-2/SM_FlipBoardLR.SM_FlipBoardLR") (== _staticmesh_2 "/Game/BoxesLike/StaticMesh/Box2-2/SM_FlipBoardTB.SM_FlipBoardTB")))
  (if LisTandRisF
    (if _returnvalue_2
      (`PrimitiveComponent.SetMaterial` (`local.FlipPanel`) 3 "/Game/BoxesLike/Materials/M_YellowLightMetal.M_YellowLightMetal")
      (elif _returnvalue
        (`PrimitiveComponent.SetMaterial` (`local.FlipPanel`) 2 "/Game/BoxesLike/Materials/M_YellowLightMetal.M_YellowLightMetal")
        (else
          (`PrimitiveComponent.SetMaterial` (`local.FlipPanel`) 0 "/Game/BoxesLike/Materials/M_YellowLightMetal.M_YellowLightMetal"))))
    (elif _returnvalue_2
      (`PrimitiveComponent.SetMaterial` (`local.FlipPanel`) 3 "/Game/BoxesLike/Materials/M_BlueLightMetal.M_BlueLightMetal")
      (elif _returnvalue
        (`PrimitiveComponent.SetMaterial` (`local.FlipPanel`) 2 "/Game/BoxesLike/Materials/M_BlueLightMetal.M_BlueLightMetal")
        (else
          (`PrimitiveComponent.SetMaterial` (`local.FlipPanel`) 0 "/Game/BoxesLike/Materials/M_BlueLightMetal.M_BlueLightMetal"))))))

(fn `FlipMove`
  (params (FlipPanel :type "StaticMeshComponent Object Reference") (TimelineValue :type "Float (double-precision)") (FlipDirection :type "Float (double-precision)"))
  (locals (MoveZ :type "Float (double-precision)" :default 2.0))
  (bind _staticmesh (`StaticMeshComponent.StaticMesh` FlipPanel))
  (bind (_relativelocation_x _relativelocation_y) (`KismetMathLibrary.BreakVector` (`SceneComponent.RelativeLocation` FlipPanel)))
  (if (or (== _staticmesh "/Game/BoxesLike/StaticMesh/Box2-2/SM_FlipBoardLL.SM_FlipBoardLL") (== _staticmesh "/Game/BoxesLike/StaticMesh/Box2-2/SM_FlipBoardRR.SM_FlipBoardRR"))
    (set `local.MoveZ` 2.5)
    (else
      (set `local.MoveZ` 2.0)))
  (`SceneComponent.K2_SetRelativeLocationAndRotation` FlipPanel (`KismetMathLibrary.MakeVector` _relativelocation_x _relativelocation_y (`local.MoveZ`)) (`KismetMathLibrary.RLerp` (`KismetMathLibrary.MakeRotator` (* FlipDirection 180.0)) (struct) TimelineValue) false false))

(fn `UserConstructionScript`)