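; Left gear set actor for the Box2-2 level that starts spinning once the BP_RightCogWheel actor flags KeyUsed.
; A one-shot on Tick switches four Niagara effects to light blue and plays a timeline that rotates four gears in alternating directions.
; When the timeline finishes, RotatingMovement takes over the top gear and SpinStart is set.
; Tick continually copies or negates the top gear's rotation onto the other three.
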(event `self.ReceiveBeginPlay`
  ;[1 1 1] 우측면 톱니바퀴 회전 애니메이션 종료 감지용 변수 저장
  (bind _outactors (`GameplayStatics.GetAllActorsOfClass` "/Game/BoxesLike/BluePrints/Box2-2/BP_RightCogWheel.BP_RightCogWheel_C"))
  (set `self.RightCogWheel` (`|GetArrayItem` _outactors))
  (`MovementComponent.SetUpdatedComponent` (`self.RotatingMovement`) (`self.StylizedGearTop`)))

(event `self.ReceiveTick`
  (params (DeltaSeconds :type "Float (single-precision)"))
  (bind _relativerotation (`SceneComponent.RelativeRotation` (`self.StylizedGearTop`)))
  ;[1 1 1] 우측 톱니바퀴 속도가 최대치에 도달하면 좌측 톱니바퀴들도 돌아간다.
  (`|ExecutionSequence`
    (:`then_0`
      (if (`/Game/BoxesLike/BluePrints/Box2-2/BP_RightCogWheel.KeyUsed` (`self.RightCogWheel`))
        (`/Engine/EditorBlueprintResources/StandardMacros.DoOnce` false
          (:`Completed`
            (`NiagaraComponent.SetAsset` (`self.NiagaraB`) "/Game/BoxesLike/VFX/Box2-2/VFS_GearLightBlue.VFS_GearLightBlue" true)
            (`NiagaraComponent.SetAsset` (`self.NiagaraT`) "/Game/BoxesLike/VFX/Box2-2/VFS_GearLightBlue.VFS_GearLightBlue" true)
            (`NiagaraComponent.SetAsset` (`self.NiagaraTL`) "/Game/BoxesLike/VFX/Box2-2/VFS_GearLightBlue.VFS_GearLightBlue" true)
            (`NiagaraComponent.SetAsset` (`self.NiagaraBR`) "/Game/BoxesLike/VFX/Box2-2/VFS_GearLightBlue.VFS_GearLightBlue" true) ; 이펙트 주황에서 파랑으로
            (bind (_direction _value) (`Timeline|Timeline`) ; 갑자기 최대속도로 돌면 이상하니까\n천천히 속도 UP
              (:`Update`
                (`SceneComponent.K2_SetRelativeRotation` (`self.StylizedGearBottomRight`) (`KismetMathLibrary.MakeRotator` (* _value 240.0)) false false)
                (`SceneComponent.K2_SetRelativeRotation` (`self.StylizedGearTop`) (`KismetMathLibrary.MakeRotator` (* _value 240.0)) false false)
                (`SceneComponent.K2_SetRelativeRotation` (`self.StylizedGearBottom`) (`KismetMathLibrary.MakeRotator` (* _value -240.0)) false false)
                (`SceneComponent.K2_SetRelativeRotation` (`self.StylizedGearTopLeft`) (`KismetMathLibrary.MakeRotator` (* _value -240.0)) false false))
              (:`Finished`
                (`ActorComponent.Activate` (`self.RotatingMovement`) false)
                (set `self.SpinStart` true)))))))
    (:`then_1`
      (`SceneComponent.K2_SetRelativeRotation` (`self.StylizedGearBottom`) (* _relativerotation -1.0) false false)
      (`SceneComponent.K2_SetRelativeRotation` (`self.StylizedGearTopLeft`) (* _relativerotation -1.0) false false)
      (`SceneComponent.K2_SetRelativeRotation` (`self.StylizedGearBottomRight`) _relativerotation false false))))

(fn `UserConstructionScript`)