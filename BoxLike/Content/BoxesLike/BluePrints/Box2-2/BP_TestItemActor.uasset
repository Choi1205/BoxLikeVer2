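; BP_TestItemActor is an item actor that can be picked up or inspected by rotating its mesh, set from InspectItemShape at construction.
; StartInspect moves input from the inspector to this actor, where left-drag applies yaw and pitch.
; Right-click restores the inspector's input and calls EndInspectMouse on the first-person character.
; GetItem returns the item's data and triggers destruction, delayed briefly so the return values survive.
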(event `DestoryItem`
  ;[1 1 1] 아이템 획득시 딜레이를 줘서 액터 삭제 전 리턴값을 줄 시간을 얻음.
  ; 액터 삭제 전 획득 애니메이션 삽입 가능
  (`KismetSystemLibrary.Delay` 0.2)
  (`self.K2_DestroyActor`))

(event `StartInspect`
  (params (Inspector :type "Pawn Object Reference"))
  (bind _returnvalue (`GameplayStatics.GetPlayerController` 0))
  ;[1 1 1] 아이템 상세 확인 시작/종료 부분. 상세 확인을 시작하면 플레이어 캐릭터에 있던 컨트롤을 생성된 이 액터로 옮긴다.
  (`self.DisableInput` Inspector _returnvalue)
  (`self.EnableInput` _returnvalue)
  (set `self.IsInspecting` true))

(event `Key|RightMouseButton`
  (params (Key :type "Key Structure"))
  (bind _returnvalue (`GameplayStatics.GetPlayerController` 0))
  ;[1 1 1] 아이템 상세 확인 시작/종료 부분. 상세 확인을 시작하면 플레이어 캐릭터에 있던 컨트롤을 생성된 이 액터로 옮긴다.
  (:`Pressed`
    (`self.DisableInput` _returnvalue)
    (`self.EnableInput` (stale `StartInspect` Inspector) _returnvalue)
    (bind _asbp_first_person_character (cast `/Game/FirstPerson/Blueprints/BP_FirstPersonCharacter` (`GameplayStatics.GetPlayerCharacter` 0)))
    (`/Game/FirstPerson/Blueprints/BP_FirstPersonCharacter.EndInspectMouse` _asbp_first_person_character)))

(event `InputAxisKey|MouseX`
  (params (AxisValue :type "Float (single-precision)"))
  ;[1 1 1] 마우스를 드래그하면 이 스태틱 매쉬가 회전한다.
  (if (and (`PlayerController.IsInputKeyDown` (`GameplayStatics.GetPlayerController` 0) "LeftMouseButton") (`self.IsInspecting`))
    (`SceneComponent.K2_SetRelativeRotation` (`self.StaticMesh`) (`KismetMathLibrary.ComposeRotators` (`SceneComponent.RelativeRotation` (`self.StaticMesh`)) (`KismetMathLibrary.MakeRotator` 0.0 0.0 (* AxisValue -1.0))) false false)))

(event `InputAxisKey|MouseY`
  (params (AxisValue :type "Float (single-precision)"))
  ;[1 1 1] 마우스를 드래그하면 이 스태틱 매쉬가 회전한다.
  (if (and (`PlayerController.IsInputKeyDown` (`GameplayStatics.GetPlayerController` 0) "LeftMouseButton") (`self.IsInspecting`))
    (`SceneComponent.K2_SetRelativeRotation` (`self.StaticMesh`) (`KismetMathLibrary.ComposeRotators` (`SceneComponent.RelativeRotation` (`self.StaticMesh`)) (`KismetMathLibrary.MakeRotator` 0.0 (* AxisValue -1.0))) false false)))

(fn `GetItem`
  (returns (ItemID :type Integer) (ItemName :type String) (ItemTexture :type "Texture2D Object Reference") (ItemStaticMesh :type "StaticMesh Object Reference"))
  ;[1 1 1] 리턴값이 있으므로 딜레이를 줘서 값이 소실되는 것을 방지
  (`self.DestoryItem`)
  (return (`self.ItemID`) (`self.ItemName`) (`self.ItemTexture`) (`self.ItemStaticMesh`)))

(fn `UserConstructionScript`
  (`StaticMeshComponent.SetStaticMesh` (`self.StaticMesh`) (`self.InspectItemShape`)))