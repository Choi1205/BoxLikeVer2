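; BP_SparkPoint is a puzzle actor that links the lever puzzle to a cover item-use step and key glass reveal.
; BeginPlay finds the lever hole and matching item-use point by NeedItemID, disabling the latter's collision.
; Tick polls the lever, then shuts off sparks and shifts and enables that point.
; Once used, the point is destroyed, and its invalid reference triggers chained cover and glass timelines with player input disabled.
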(event `self.ReceiveBeginPlay`
  (`|ExecutionSequence`
    (:`then_0`
      ;[1 1 1] 아이템 사용 포인트 변수로 저장
      (bind _outactors (`GameplayStatics.GetAllActorsWithInterface` "/Game/BoxesLike/BPInterface/ItemUsingPoint.ItemUsingPoint_C"))
      (for _array_element _outactors
        (bind _asbp_item_using_point (cast `/Game/BoxesLike/BluePrints/TestBoxBP/BP_ItemUsingPoint` _array_element))
        (if (== (`/Game/BoxesLike/BluePrints/TestBoxBP/BP_ItemUsingPoint.NeedItemID` _asbp_item_using_point) 22)
          (set `self.Cover` _array_element)
          (`PrimitiveComponent.SetCollisionEnabled` (`/Game/BoxesLike/BluePrints/TestBoxBP/BP_ItemUsingPoint.Box` _asbp_item_using_point) "NoCollision"))))
    (:`then_1`
      ;[1 1 1] 이전 퍼즐(레버 당기기) 변수로 저장
      (bind _outactors_2 (`GameplayStatics.GetAllActorsOfClass` "/Game/BoxesLike/BluePrints/Box2-2/BP_LeverHole.BP_LeverHole_C"))
      (set `self.LeverHole` (`|GetArrayItem` _outactors_2)))))

(event `self.ReceiveTick`
  (params (DeltaSeconds :type "Float (single-precision)"))
  (bind _cover (`self.Cover`))
  (bind _cover_2 (`self.Cover`))
  (bind _sm_rightpincover (`self.SM_RightPinCover`))
  (bind (_returnvalue_x _returnvalue_y _returnvalue_z) (`KismetMathLibrary.BreakVector` (`self.K2_GetActorLocation` _cover_2)))
  (bind (_relativelocation_x _relativelocation_y _relativelocation_z) (`KismetMathLibrary.BreakVector` (`SceneComponent.RelativeLocation` _sm_rightpincover)))
  (bind (_relativelocation_x_2 _relativelocation_y_2 _relativelocation_z_2) (`KismetMathLibrary.BreakVector` (`SceneComponent.RelativeLocation` (`self.SM_KeyGlass`))))
  (`|ExecutionSequence`
    (:`then_0`
      ;[1 1 1] 레버를 당겼으면 스파크를 끄고 잠겨있던 아이템 사용포인트가 사용 가능하게 됨
      (if (`/Game/BoxesLike/BluePrints/Box2-2/BP_LeverHole.LeverMoveEnd` (`self.LeverHole`))
        (`/Engine/EditorBlueprintResources/StandardMacros.DoOnce` false
          (:`Completed`
            (`self.K2_SetActorLocation` _cover_2 (`KismetMathLibrary.MakeVector` _returnvalue_x (+ _returnvalue_y 6.0) _returnvalue_z) false false)
            (bind _asbp_item_using_point (cast `/Game/BoxesLike/BluePrints/TestBoxBP/BP_ItemUsingPoint` (`self.Cover`)))
            (`PrimitiveComponent.SetCollisionEnabled` (`/Game/BoxesLike/BluePrints/TestBoxBP/BP_ItemUsingPoint.Box` _asbp_item_using_point) "QueryAndPhysics")
            (`ActorComponent.Deactivate` (`self.ParticleSystem1`))
            (`ActorComponent.Deactivate` (`self.ParticleSystem2`))))))
    (:`then_1`
      ;[1 1 1] 커버 사용시 애니메이션
      (`/Engine/EditorBlueprintResources/StandardMacros.IsValid` _cover
        (:`Is Valid`
          (bind _asbp_item_using_point_2 (cast `/Game/BoxesLike/BluePrints/TestBoxBP/BP_ItemUsingPoint` _cover))
          (if (`/Game/BoxesLike/BluePrints/TestBoxBP/BP_ItemUsingPoint.ItUsed` _asbp_item_using_point_2)
            (`self.K2_DestroyActor` _cover)))
        (:`Is Not Valid`
          (`/Engine/EditorBlueprintResources/StandardMacros.DoOnce` false
            (:`Completed`
              (`self.DisableInput` (`GameplayStatics.GetPlayerPawn` 0) (`GameplayStatics.GetPlayerController` 0))
              (`StaticMeshComponent.SetStaticMesh` _sm_rightpincover "/Game/BoxesLike/StaticMesh/Box2-2/SM_RightPinCover.SM_RightPinCover")
              (set `self.CoverStartLocationY` _relativelocation_y)
              (bind (_direction _value) (`Timeline|Timeline`)
                (:`Update`
                  (`SceneComponent.K2_SetRelativeLocation` (`self.SM_RightPinCover`) (`KismetMathLibrary.MakeVector` _relativelocation_x (+ (* _value -6.0) (`self.CoverStartLocationY`)) _relativelocation_z) false false))
                (:`Finished`
                  (set `self.GlassStartLocationZ` _relativelocation_z_2)
                  (bind (_direction_2 _value_2) (`Timeline|KeyGlassUP`)
                    (:`Update`
                      (`SceneComponent.K2_SetRelativeLocation` (`self.SM_KeyGlass`) (`KismetMathLibrary.MakeVector` _relativelocation_x_2 _relativelocation_y_2 (+ (* _value_2 19.0) (`self.GlassStartLocationZ`))) false false)
                      (set `self.KeyGlassOpen` true))
                    (:`Finished`
                      (`self.EnableInput` (`GameplayStatics.GetPlayerPawn` 0) (`GameplayStatics.GetPlayerController` 0)))))))))))))

(fn `UserConstructionScript`)