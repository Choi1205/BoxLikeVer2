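; Lever socket puzzle actor that takes a lever item and lets the player pull it down by mouse drag.
; BeginPlay finds the matching ItemUsingPoint by item ID; Tick watches for its use, destroys it and plays a timeline inserting the lever mesh with player input disabled.
; BlockMoving hands input from the mover to this actor until left-mouse release.
; Downward drags lower the lever to a clamped end position, setting LeverMoveEnd.
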(event `self.ReceiveBeginPlay`
  ;[1 1 1] 아이템 사용 포인트 연결
  (bind _outactors (`GameplayStatics.GetAllActorsWithInterface` "/Game/BoxesLike/BPInterface/ItemUsingPoint.ItemUsingPoint_C"))
  (for _array_element _outactors
    (bind _asbp_item_using_point (cast `/Game/BoxesLike/BluePrints/TestBoxBP/BP_ItemUsingPoint` _array_element))
    (if (== (`/Game/BoxesLike/BluePrints/TestBoxBP/BP_ItemUsingPoint.NeedItemID` _asbp_item_using_point) 25)
      (set `self.Lever` _array_element))))

(event `self.ReceiveTick`
  (params (DeltaSeconds :type "Float (single-precision)"))
  (bind _lever (`self.Lever`))
  (bind _levermakepoint (`self.LeverMakePoint`))
  (bind (_relativelocation_x _relativelocation_y _relativelocation_z) (`KismetMathLibrary.BreakVector` (`SceneComponent.RelativeLocation` _levermakepoint)))
  ;[1 1 1] 레버 사용시 레버 꽃힘 연출
  (`/Engine/EditorBlueprintResources/StandardMacros.IsValid` _lever
    (:`Is Valid`
      (bind _asbp_item_using_point (cast `/Game/BoxesLike/BluePrints/TestBoxBP/BP_ItemUsingPoint` _lever))
      (if (`/Game/BoxesLike/BluePrints/TestBoxBP/BP_ItemUsingPoint.ItUsed` _asbp_item_using_point)
        (`self.K2_DestroyActor` _lever)
        (`self.DisableInput` (`GameplayStatics.GetPlayerPawn` 0) (`GameplayStatics.GetPlayerController` 0)) ; IsNotValid에서 이어놓은 경우도 있다.\n이 경우와 완전히 동일
        (`StaticMeshComponent.SetStaticMesh` _levermakepoint "/Game/BoxesLike/StaticMesh/Box2-2/SM_PushLever.SM_PushLever")
        (set `self.LeverStartLocation X` _relativelocation_x)
        (bind (_direction _value) (`Timeline|LeverInsert`)
          (:`Update`
            (`SceneComponent.K2_SetRelativeLocation` (`self.LeverMakePoint`) (`KismetMathLibrary.MakeVector` (+ (* _value 3.0) (`self.LeverStartLocation X`)) _relativelocation_y _relativelocation_z) false false))
          (:`Finished`
            (`self.EnableInput` (`GameplayStatics.GetPlayerPawn` 0) (`GameplayStatics.GetPlayerController` 0))))))))

(event `/Game/BoxesLike/BPInterface/BlockMoving.Block Moving`
  (params (Mover :type "Pawn Object Reference") (ClickPoint :type "Vector Structure") (LookingComponentPoint :type "PrimitiveComponent Object Reference"))
  (bind _returnvalue (`GameplayStatics.GetPlayerController` 0))
  ;[1 1 1] 레버 이동 전후 컨트롤 이동
  (if (== LookingComponentPoint (`self.LeverMakePoint`))
    (`self.DisableInput` Mover _returnvalue)
    (`self.EnableInput` _returnvalue)))

(event `Key|LeftMouseButton`
  (params (Key :type "Key Structure"))
  (bind _returnvalue (`GameplayStatics.GetPlayerController` 0))
  ;[1 1 1] 레버 이동 전후 컨트롤 이동
  (:`Released`
    (`self.DisableInput` _returnvalue)
    (`self.EnableInput` (stale `/Game/BoxesLike/BPInterface/BlockMoving.Block Moving` Mover) _returnvalue)))

(event `InputAxisKey|MouseY`
  (params (AxisValue :type "Float (single-precision)"))
  (bind _relativelocation_x (`KismetMathLibrary.BreakVector` (`SceneComponent.RelativeLocation` (`self.LeverMakePoint`))))
  (bind (_relativelocation_x_2 _relativelocation_y _relativelocation_z) (`KismetMathLibrary.BreakVector` (`SceneComponent.RelativeLocation` (`self.LeverMakePoint`))))
  (bind _returnvalue (+ _relativelocation_z (* AxisValue 0.5)))
  ;[1 1 1] 마우스를 드래그하면 이 스태틱 매쉬가 이동한다. 원하는 축/방향에 맞춰서 X/Y , XYZ 연결을 조정
  (if (and (< AxisValue 0.0) (< _relativelocation_x 98.0) (`PlayerController.IsInputKeyDown` (`GameplayStatics.GetPlayerController` 0) "LeftMouseButton"))
    (`SceneComponent.K2_SetRelativeLocation` (`self.LeverMakePoint`) (`KismetMathLibrary.MakeVector` _relativelocation_x_2 _relativelocation_y _returnvalue) false false)
    (if (<= _returnvalue -8.0)
      (set `self.LeverMoveEnd` true)
      (`SceneComponent.K2_SetRelativeLocation` (`self.LeverMakePoint`) (`KismetMathLibrary.MakeVector` _relativelocation_x_2 _relativelocation_y -8.0) false false) ; 레버 위치 정리
    )))

(fn `UserConstructionScript`)