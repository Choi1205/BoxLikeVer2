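; Multi-stage table puzzle actor with roll locks, sliding doors and a battery-powered bulb-sorting puzzle.
; Mouse drags move input to the actor to rotate both locks, which snap near zero and then let the doors slide.
; Tick polls the battery use point found in construction, then animates insertion and rotates the puzzle in.
; Switches swap adjacent array entries, recolor Niagara lights and, on matching the answer, slide AnswerPlace and complete the puzzle.
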(event `self.ReceiveTick`
  (params (DeltaSeconds :type "Float (single-precision)"))
  (bind _batteryusingpoint (`self.BatteryUsingPoint`))
  ;[1 1 1] 배터리 사용 후 정렬퍼즐 등장
  (`/Engine/EditorBlueprintResources/StandardMacros.IsValid` _batteryusingpoint ; 배터리 사용됬는지 체크
    (:`Is Valid`
      (bind _asbp_item_using_point (cast `/Game/BoxesLike/BluePrints/TestBoxBP/BP_ItemUsingPoint` _batteryusingpoint))
      (if (`/Game/BoxesLike/BluePrints/TestBoxBP/BP_ItemUsingPoint.ItUsed` _asbp_item_using_point)
        (set `self.BatteryUsed` true)
        (`self.K2_DestroyActor` _batteryusingpoint) ; 사용된 포인트는 제거
      ))
    (:`Is Not Valid`
      (`/Engine/EditorBlueprintResources/StandardMacros.DoOnce` false
        (:`Completed`
          (`self.BatteryMove`))))))

(event `BatteryMove`
  (bind (_relativelocation_x _relativelocation_y _relativelocation_z) (`KismetMathLibrary.BreakVector` (`SceneComponent.RelativeLocation` (`self.Battery`))))
  ;[1 1 1] 배터리를 사용하면 배터리가 슬롯에 꽃히고, 정렬 퍼즐이 회전하며 등장하는 연출
  (`self.DisableInput` (`GameplayStatics.GetPlayerPawn` 0) (`GameplayStatics.GetPlayerController` 0))
  (`StaticMeshComponent.SetStaticMesh` (`self.Battery`) "/Game/BoxesLike/Assets/9VBattery/9V_Battery.9V_Battery")
  (set `self.BatteryStartLocX` _relativelocation_x)
  (bind (_direction _value) (`Timeline|BatteryMovement`)
    (:`Update`
      (`SceneComponent.K2_SetRelativeLocation` (`self.Battery`) (`KismetMathLibrary.MakeVector` (+ (* _value 8.0) (`self.BatteryStartLocX`)) _relativelocation_y _relativelocation_z) false false))
    (:`Finished`
      (`GameplayStatics.PlaySound2D` "/Game/BoxesLike/Sound/SE/Choi/SEC_stun-gun-zap_Cue.SEC_stun-gun-zap_Cue" 1.0 1.0 0.0 null null)
      (`KismetSystemLibrary.Delay` 0.5)
      (set `self.PuzzleStartRotation` (`SceneComponent.RelativeRotation` (`self.PuzzleBody`)))
      (`GameplayStatics.PlaySound2D` "/Game/BoxesLike/Sound/SE/Choi/SEC_clicky_wheel_2_Cue.SEC_clicky_wheel_2_Cue" 1.0 1.0 0.0 null null)
      (bind (_direction_2 _value_2) (`Timeline|Timeline`)
        (:`Update`
          (`SceneComponent.K2_SetRelativeRotation` (`self.PuzzleBody`) (`KismetMathLibrary.RLerp` (struct) (struct :`Pitch` 180.0) _value_2 true) false false))
        (:`Finished`
          (`self.BulbsON`)
          (`self.EnableInput` (`GameplayStatics.GetPlayerPawn` 0) (`GameplayStatics.GetPlayerController` 0)))))))

(event `/Game/BoxesLike/BPInterface/BlockMoving.Block Moving`
  (params (Mover :type "Pawn Object Reference") (ClickPoint :type "Vector Structure") (LookingComponentPoint :type "PrimitiveComponent Object Reference"))
  (bind _returnvalue (`GameplayStatics.GetPlayerController` 0))
  ;[1 1 1] 아이템 상세 확인 시작/종료 부분. 상세 확인을 시작하면 플레이어 캐릭터에 있던 컨트롤을 생성된 이 액터로 옮긴다.
  (set `self.Looking Component Point` LookingComponentPoint)
  (bind (_rollordoor _isrool) (`self.FindClickPlace`)) ; 도어를 클릭했는지, 롤을 클릭했는지 확인
  (if _rollordoor
    (if _isrool
      (set `self.RollISTandPushISF` true)
      (else
        (set `self.RollISTandPushISF` false)))
    (`self.DisableInput` Mover _returnvalue)
    (`self.EnableInput` _returnvalue)))

(event `Key|LeftMouseButton`
  (params (Key :type "Key Structure"))
  (bind _returnvalue (`GameplayStatics.GetPlayerController` 0))
  ;[1 1 1] 드래그 종료시 좌/우 Roll도어의 위치가 0에 근접하면 자동으로 0으로 맞춰준다.
  (:`Released`
    (bind _result (`self.LeftRollDoorRotateFitCheak`)) ; 왼쪽 도어가 정위치에 근접했는지 체크
    (if _result
      (bind (_direction _rotaterate) (`Timeline|LeftRollmove`)
        (:`Update`
          (`self.RollDoorFitMoving` (`self.LeftRotateEndValue`) _rotaterate) ; 정위치로 이동시킨다
        )
        (:`Finished`
          (set `self.RotateNotCompleteL` false)
          (`GameplayStatics.PlaySound2D` "/Game/BoxesLike/Sound/SE/Choi/SEC_gun_hit_1_Cue.SEC_gun_hit_1_Cue" 1.0 1.0 0.0 null null :!label _label)
          ;[1 1 1] 아이템 상세 확인 시작/종료 부분. 상세 확인을 시작하면 플레이어 캐릭터에 있던 컨트롤을 생성된 이 액터로 옮긴다.
          (`self.DisableInput` _returnvalue :!label _label_2)
          (`self.EnableInput` (stale `/Game/BoxesLike/BPInterface/BlockMoving.Block Moving` Mover) _returnvalue)))
      (else
        (bind _result_2 (`self.RightRollDoorRotateFitCheak`))
        (if _result_2
          (bind (_direction_2 _rotaterate_2) (`Timeline|RightRollmove`)
            (:`Update`
              (`self.RollDoorFitMoving` (`self.RightRotateEndValue`) _rotaterate_2))
            (:`Finished`
              (set `self.RotateNotCompleteR` false)
              (goto _label)))
          (else
            (goto _label_2)))))))

(event `InputAxisKey|MouseX`
  (params (AxisValue :type "Float (single-precision)"))
  ;[1 1 1] 마우스를 드래그하면 이 스태틱 매쉬가 이동한다. 원하는 축/방향에 맞춰서 X/Y , XYZ 연결을 조정
  (set `self.Axis ValueX` AxisValue)
  (bind _conditionresult (`self.DoorMoveCondition`)) ; 도어 이동가능한지 체크
  (if _conditionresult
    (bind _newvector (`self.MakeDoorComponentVector` (`self.Looking Component Point`))) ; 도어 이동백터를 계산한다
    (`SceneComponent.K2_SetRelativeLocation` (`self.Looking Component Point`) _newvector false false)))

(event `InputAxisKey|MouseY`
  (params (AxisValue :type "Float (single-precision)"))
  (bind (_relativerotation_roll _relativerotation_pitch _relativerotation_yaw) (`KismetMathLibrary.BreakRotator` (`SceneComponent.RelativeRotation` (`self.Looking Component Point`))))
  ;[1 1 1] 마우스를 드래그하면 이 스태틱 매쉬가 이동한다. 원하는 축/방향에 맞춰서 X/Y , XYZ 연결을 조정
  (if (and (`self.RollISTandPushISF`) (`PlayerController.IsInputKeyDown` (`GameplayStatics.GetPlayerController` 0) "LeftMouseButton"))
    (`SceneComponent.K2_AddLocalRotation` (`self.Looking Component Point`) (`KismetMathLibrary.MakeRotator` 0.0 (* AxisValue -1.0)) false false)
    (if (== (`self.Looking Component Point`) (`self.SM_TableRollLockLeft`))
      (set `self.LeftRotateEndValue` _relativerotation_pitch)
      (set `self.LeftRotateYValue` _relativerotation_yaw)
      (else
        (set `self.RightRotateEndValue` _relativerotation_pitch)
        (set `self.RightRotateYValue` _relativerotation_yaw)))))

(event `self.SM_TablePuzzleSwitch01.OnClicked`
  (params (TouchedComponent :type "PrimitiveComponent Object Reference") (ButtonPressed :type "Key Structure"))
  (bind (_relativelocation_x _relativelocation_y _relativelocation_z) (`KismetMathLibrary.BreakVector` (`SceneComponent.RelativeLocation` (`self.AnswerPlace`))))
  ;[1 1 1] 버블정렬 퍼즐 구간
  (`KismetArrayLibrary.Array_Swap` (`self.AnswerArrey`) 0 1)
  (for (_array_element _array_index) (`self.AnswerArrey`) :!label _label_3
    (if (not (`self.PuzzleComplete`))
      (`self.ChangeAndCheak` _array_element _array_index) ; 전극색을 바꿔주고 배열일치를 확인
    ))
  (`GameplayStatics.PlaySound2D` "/Game/BoxesLike/Sound/SE/Choi/SEC_stun-gun-zap_Cue.SEC_stun-gun-zap_Cue" 1.0 1.0 0.0 null null)
  (if (`self.NumberNotSame`)
    (set `self.NumberNotSame` false)
    (else
      (`/Engine/EditorBlueprintResources/StandardMacros.DoOnce` false
        (:`Completed`
          (`self.DisableInput` (`GameplayStatics.GetPlayerPawn` 0) (`GameplayStatics.GetPlayerController` 0))
          (set `self.PinStartLocationX` _relativelocation_x)
          (bind (_direction _movingrate) (`Timeline|CorrectAnswer`)
            (:`Update`
              (`SceneComponent.K2_SetRelativeLocation` (`self.AnswerPlace`) (`KismetMathLibrary.MakeVector` (+ (* _movingrate 1.5) (`self.PinStartLocationX`)) _relativelocation_y _relativelocation_z) false false))
            (:`Finished`
              (`self.EnableInput` (`GameplayStatics.GetPlayerPawn` 0) (`GameplayStatics.GetPlayerController` 0))
              (`self.BulbsOFF`)
              (`GameplayStatics.PlaySound2D` "/Game/BoxesLike/Sound/SE/Choi/SEC_zap_Cue.SEC_zap_Cue" 1.0 1.0 0.0 null null)
              (`KismetSystemLibrary.Delay` 1.0) ; 퍼즐 완료되면 효과음을 켜면서 잠깐 멈추기
              (set `self.PuzzleComplete` true) ; 퍼즐 완료
            )))))))

(event `self.SM_TablePuzzleSwitch12.OnClicked`
  (params (TouchedComponent :type "PrimitiveComponent Object Reference") (ButtonPressed :type "Key Structure"))
  ;[1 1 1] 버블정렬 퍼즐 구간
  (`KismetArrayLibrary.Array_Swap` (`self.AnswerArrey`) 1 2)
  (goto _label_3))

(event `self.SM_TablePuzzleSwitch23.OnClicked`
  (params (TouchedComponent :type "PrimitiveComponent Object Reference") (ButtonPressed :type "Key Structure"))
  ;[1 1 1] 버블정렬 퍼즐 구간
  (`KismetArrayLibrary.Array_Swap` (`self.AnswerArrey`) 2 3)
  (goto _label_3))

(event `self.SM_TablePuzzleSwitch34.OnClicked`
  (params (TouchedComponent :type "PrimitiveComponent Object Reference") (ButtonPressed :type "Key Structure"))
  ;[1 1 1] 버블정렬 퍼즐 구간
  (`KismetArrayLibrary.Array_Swap` (`self.AnswerArrey`) 3 4)
  (goto _label_3))

(event `self.SM_TablePuzzleSwitch45.OnClicked`
  (params (TouchedComponent :type "PrimitiveComponent Object Reference") (ButtonPressed :type "Key Structure"))
  ;[1 1 1] 버블정렬 퍼즐 구간
  (`KismetArrayLibrary.Array_Swap` (`self.AnswerArrey`) 4 5)
  (goto _label_3))

(fn `BulbsOFF`
  (`ActorComponent.Deactivate` (`self.ALight0`))
  (`ActorComponent.Deactivate` (`self.ALight1`))
  (`ActorComponent.Deactivate` (`self.ALight2`))
  (`ActorComponent.Deactivate` (`self.ALight3`))
  (`ActorComponent.Deactivate` (`self.ALight4`))
  (`ActorComponent.Deactivate` (`self.ALight5`)))

(fn `BulbsON`
  (`ActorComponent.Activate` (`self.ALight0`) false)
  (`ActorComponent.Activate` (`self.Light5`) false)
  (`ActorComponent.Activate` (`self.Light3`) false)
  (`ActorComponent.Activate` (`self.Light1`) false)
  (`ActorComponent.Activate` (`self.Light2`) false)
  (`ActorComponent.Activate` (`self.Light4`) false)
  (`ActorComponent.Activate` (`self.Light0`) false)
  (`ActorComponent.Activate` (`self.ALight2`) false)
  (`ActorComponent.Activate` (`self.ALight1`) false)
  (`ActorComponent.Activate` (`self.ALight3`) false)
  (`ActorComponent.Activate` (`self.ALight5`) false)
  (`ActorComponent.Activate` (`self.ALight4`) false))

(fn `ChangeAndCheak`
  (params (ElementValue :type Integer) (IndexNum :type Integer))
  (bind _output (`|GetArrayItem` (`self.NiagaraData`) IndexNum))
  ;[1 1 1] 전극 색을 바꾸고 배열이 일치하는지 검사한다. 전극 1쌍만 바꿨어도 모든 전극을 검사함
  (switch `int` ElementValue
    (:`0`
      (`NiagaraComponent.SetAsset` _output "/Game/BoxesLike/VFX/Box2-2/VFS_BulbLight0.VFS_BulbLight0" true))
    (:`1`
      (`NiagaraComponent.SetAsset` _output "/Game/BoxesLike/VFX/Box2-2/VFS_BulbLight1.VFS_BulbLight1" true))
    (:`2`
      (`NiagaraComponent.SetAsset` _output "/Game/BoxesLike/VFX/Box2-2/VFS_BulbLight2.VFS_BulbLight2" true))
    (:`3`
      (`NiagaraComponent.SetAsset` _output "/Game/BoxesLike/VFX/Box2-2/VFS_BulbLight3.VFS_BulbLight3" true))
    (:`4`
      (`NiagaraComponent.SetAsset` _output "/Game/BoxesLike/VFX/Box2-2/VFS_BulbLight4.VFS_BulbLight4" true))
    (:`5`
      (`NiagaraComponent.SetAsset` _output "/Game/BoxesLike/VFX/Box2-2/VFS_BulbLight5.VFS_BulbLight5" true)))
  (if (not (== (`|GetArrayItem` (`self.BulbArrey`) (`local.IndexNum`)) (`|GetArrayItem` (`self.AnswerArrey`) (`local.IndexNum`))))
    (set `self.NumberNotSame` true)))

(fn `DoorMoveCondition`
  (returns (ConditionResult :type Boolean))
  (bind (_relativelocation_x _relativelocation_y) (`KismetMathLibrary.BreakVector` (`SceneComponent.RelativeLocation` (`self.Looking Component Point`))))
  ;[1 1 1] 도어 이동 가능 여부 확인
  (return (and (not (`self.RollISTandPushISF`)) (`KismetMathLibrary.BooleanNOR` (`self.RotateNotCompleteL`) (`self.RotateNotCompleteR`)) (`PlayerController.IsInputKeyDown` (`GameplayStatics.GetPlayerController` 0) "LeftMouseButton") (< (`KismetMathLibrary.Abs` _relativelocation_y) 15.0) (or (and (== (`self.Looking Component Point`) (`self.SM_TablePushDoorLeft`)) (< (`self.Axis ValueX`) 0.0)) (and (== (`self.Looking Component Point`) (`self.SM_TablePushDoorRight`)) (> (`self.Axis ValueX`) 0.0))))))

(fn `FindClickPlace`
  (returns (RollORDoor :type Boolean) (IsRool :type Boolean))
  (bind _returnvalue (or (and (== (`self.Looking Component Point`) (`self.SM_TableRollLockLeft`)) (`self.RotateNotCompleteL`)) (and (== (`self.Looking Component Point`) (`self.SM_TableRollLockRight`)) (`self.RotateNotCompleteR`))))
  (return (or (or (== (`self.Looking Component Point`) (`self.SM_TablePushDoorLeft`)) (== (`self.Looking Component Point`) (`self.SM_TablePushDoorRight`))) _returnvalue) _returnvalue))

(fn `ItemUsingPoint`
  (params (ItemID :type Integer :default 0))
  (returns (ItsUsed :type Boolean))
  (return (== ItemID 23)))

(fn `LeftRollDoorRotateFitCheak`
  (returns (Result :type Boolean))
  (bind _leftrotateendvalue (`self.LeftRotateEndValue`))
  (if (and (> 10.0 _leftrotateendvalue) (> _leftrotateendvalue -10.0) (< (`self.LeftRotateYValue`) 10.0) (`self.RotateNotCompleteL`))
    (return true)
    (else
      (return false))))

(fn `MakeDoorComponentVector`
  (params (DoorComponent :type "PrimitiveComponent Object Reference"))
  (returns (NewVector :type "Vector Structure"))
  (locals (NewYLocation :type "Float (double-precision)"))
  (bind (_relativelocation_x _relativelocation_y _relativelocation_z) (`KismetMathLibrary.BreakVector` (`SceneComponent.RelativeLocation` DoorComponent)))
  ;[1 1 1] 도어 이동위치 백터를 만들어냄. 마우스를 강하게 움직여서 15이상이 될 경우 15로 맞춰서 너무 크게 움직이지 않게 한다.
  (set `local.NewYLocation` (+ _relativelocation_y (* (`self.Axis ValueX`) 0.25)))
  (if (> (`KismetMathLibrary.Abs` (`local.NewYLocation`)) 15.0)
    (if (== DoorComponent (`self.SM_TablePushDoorLeft`))
      (set `local.NewYLocation` -15.0)
      (else
        (set `local.NewYLocation` 15.0))))
  (return (`KismetMathLibrary.MakeVector` _relativelocation_x (`local.NewYLocation`) _relativelocation_z)))

(fn `RightRollDoorRotateFitCheak`
  (returns (Result :type Boolean))
  (bind _rightrotateendvalue (`self.RightRotateEndValue`))
  (if (and (> 10.0 _rightrotateendvalue) (> _rightrotateendvalue -10.0) (< (`self.RightRotateYValue`) 10.0) (`self.RotateNotCompleteR`))
    (return true)
    (else
      (return false))))

(fn `RollDoorFitMoving`
  (params (RotateEndValue :type "Float (double-precision)") (TimeLineValue :type "Float (double-precision)"))
  (`SceneComponent.K2_SetRelativeRotation` (`self.Looking Component Point`) (`KismetMathLibrary.RLerp` (`KismetMathLibrary.MakeRotator` 0.0 RotateEndValue) (struct) TimeLineValue true) false false))

(fn `UserConstructionScript`
  (bind _niagaradata (`self.NiagaraData`))
  ;[1 1 1] ItemUsingPoint 연결
  (bind _outactors (`GameplayStatics.GetAllActorsWithInterface` "/Game/BoxesLike/BPInterface/ItemUsingPoint.ItemUsingPoint_C")) ; 배터리 사용 포인트 연결
  (for _array_element _outactors
    (bind _asbp_item_using_point (cast `/Game/BoxesLike/BluePrints/TestBoxBP/BP_ItemUsingPoint` _array_element))
    (if (== (`/Game/BoxesLike/BluePrints/TestBoxBP/BP_ItemUsingPoint.NeedItemID` _asbp_item_using_point) 23)
      (set `self.BatteryUsingPoint` _array_element)
      (`KismetArrayLibrary.Array_Set` _niagaradata 0 (`self.ALight0`))
      (`KismetArrayLibrary.Array_Set` _niagaradata 1 (`self.ALight1`))
      (`KismetArrayLibrary.Array_Set` _niagaradata 2 (`self.ALight2`))
      (`KismetArrayLibrary.Array_Set` _niagaradata 3 (`self.ALight3`))
      (`KismetArrayLibrary.Array_Set` _niagaradata 4 (`self.ALight4`))
      (`KismetArrayLibrary.Array_Set` _niagaradata 5 (`self.ALight5`)))))