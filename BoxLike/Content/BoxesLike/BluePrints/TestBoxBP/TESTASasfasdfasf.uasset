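; A test actor Blueprint with a clickable component that starts a Timeline when clicked.
; Each Timeline update writes the component's relative location back to itself unchanged, so it produces no movement.
; On finish it prints and increments a counter, then replays from the start while a boolean is true, otherwise printing a greeting.
; The graph never changes that boolean, and a counter limit check is left unconnected.
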(event `self.asdasfgsafda.OnClicked`
  (params (TouchedComponent :type "PrimitiveComponent Object Reference") (ButtonPressed :type "Key Structure"))
  (bind _asdasfgsafda (`self.asdasfgsafda`))
  (bind _asdfasdf (`self.asdfasdf`))
  (bind (_relativelocation_x _relativelocation_y _relativelocation_z) (`KismetMathLibrary.BreakVector` (`SceneComponent.RelativeLocation` _asdasfgsafda)))
  (`Timeline|Timeline` :!label _label
    (:`Update`
      (`SceneComponent.K2_SetRelativeLocation` _asdasfgsafda (`KismetMathLibrary.MakeVector` _relativelocation_x _relativelocation_y _relativelocation_z) false false))
    (:`Finished`
      (`KismetSystemLibrary.PrintString` (`KismetStringLibrary.Conv_IntToString` _asdfasdf))
      (set `self.asdfasdf` (+ _asdfasdf 1))
      (if (`self.NewVar`)
        (goto _label :!via `PlayFromStart`)
        (else
          (`KismetSystemLibrary.PrintString` "Hello"))))))

(fn `UserConstructionScript`)