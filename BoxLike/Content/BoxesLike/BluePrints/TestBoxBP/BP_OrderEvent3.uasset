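; BP_OrderEvent3 is a clickable test actor for the third stage of an ordered event chain, gated on earlier stages.
; On BeginPlay it caches the first two BP_OrderEvent2 actors and the first BP_OrderEvent1 found in the level.
; Clicking its Box toggles its TestFlag and particle system on or off, but only while all three cached actors have their TestFlag set.
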(event `self.ReceiveBeginPlay`
  (bind _outactors (`GameplayStatics.GetAllActorsOfClass` "/Game/BoxesLike/BluePrints/TestBoxBP/BP_OrderEvent2.BP_OrderEvent2_C"))
  (set `self.BeforeEventActor1` (`|GetArrayItem` _outactors))
  (set `self.BeforeEventActor2` (`|GetArrayItem` _outactors 1))
  (bind _outactors_2 (`GameplayStatics.GetAllActorsOfClass` "/Game/BoxesLike/BluePrints/TestBoxBP/BP_OrderEvent1.BP_OrderEvent1_C"))
  (set `self.FirstEventActor` (`|GetArrayItem` _outactors_2)))

(event `self.Box.OnClicked`
  (params (TouchedComponent :type "PrimitiveComponent Object Reference") (ButtonPressed :type "Key Structure"))
  (bind _particlesystem (`self.ParticleSystem`))
  (if (and (`/Game/BoxesLike/BluePrints/TestBoxBP/BP_OrderEvent2.TestFlag` (`self.BeforeEventActor1`)) (`/Game/BoxesLike/BluePrints/TestBoxBP/BP_OrderEvent2.TestFlag` (`self.BeforeEventActor2`)) (`/Game/BoxesLike/BluePrints/TestBoxBP/BP_OrderEvent1.TestFlag` (`self.FirstEventActor`)))
    (if (`self.TestFlag`)
      (set `self.TestFlag` false)
      (`ActorComponent.Deactivate` _particlesystem)
      (else
        (set `self.TestFlag` true)
        (`ActorComponent.Activate` _particlesystem false)))))

(fn `UserConstructionScript`)