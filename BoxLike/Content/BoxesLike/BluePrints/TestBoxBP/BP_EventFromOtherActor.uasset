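; BP_EventFromOtherActor is a test actor that switches its particle system on or off based on another actor's orientation.
; On BeginPlay it caches the first BP_RotatingBlock found in the level and deactivates its own particles.
; Every Tick it polls the world rotation of that block's Niagara component, activating particles inside a pitch window with yaw below a limit and deactivating them otherwise.
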(event `self.ReceiveBeginPlay`
  (bind _outactors (`GameplayStatics.GetAllActorsOfClass` "/Game/BoxesLike/BluePrints/TestBoxBP/BP_RotatingBlock.BP_RotatingBlock_C"))
  (set `self.TriggerActor` (`|GetArrayItem` _outactors))
  (`ActorComponent.Deactivate` (`self.ParticleSystem`)))

(event `self.ReceiveTick`
  (params (DeltaSeconds :type "Float (single-precision)"))
  (bind _particlesystem (`self.ParticleSystem`))
  (bind (_returnvalue_roll _returnvalue_pitch _returnvalue_yaw) (`KismetMathLibrary.BreakRotator` (`SceneComponent.K2_GetComponentRotation` (`/Game/BoxesLike/BluePrints/TestBoxBP/BP_RotatingBlock.Niagara` (`self.TriggerActor`)))))
  (if (and (> _returnvalue_pitch 40.0) (< _returnvalue_pitch 50.0) (< _returnvalue_yaw 90.0))
    (`ActorComponent.Activate` _particlesystem false)
    (else
      (`ActorComponent.Deactivate` _particlesystem))))

(fn `UserConstructionScript`)