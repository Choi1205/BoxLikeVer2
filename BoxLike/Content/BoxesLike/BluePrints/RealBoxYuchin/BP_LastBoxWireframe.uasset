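; BP_LastBoxWireframe is an item-use point on the last puzzle box that animates a compass and stops the box's globe.
; ItemUsingPoint reports whether the item matches NeedItemID but starts the animation either way.
; A timeline slides CompassAnim into view, calling StopGlobe on the BP_LastBoxGlobe cached at BeginPlay through a delay on its update.
; Tick only debug-prints compass overlaps with PendantCollision; FindPendant is an unused stub.
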(event `self.ReceiveBeginPlay`
  (`SceneComponent.SetVisibility` (`self.CompassAnim`) false false)
  (bind _outactors (`GameplayStatics.GetAllActorsOfClass` "/Game/BoxesLike/BluePrints/RealBoxYuchin/BP_LastBoxGlobe.BP_LastBoxGlobe_C"))
  (set `self.LastBxVar` (`|GetArrayItem` _outactors)))

(event `CompassAnimStart`
  (`SceneComponent.SetVisibility` (`self.CompassAnim`) true false)
  (bind (_direction _cp) (`Timeline|Compass`)
    (:`Update`
      (`SceneComponent.K2_SetRelativeLocation` (`self.CompassAnim`) (`KismetMathLibrary.MakeVector` _cp) false false)
      (`KismetSystemLibrary.Delay` 1.5)
      (`/Game/BoxesLike/BluePrints/RealBoxYuchin/BP_LastBoxGlobe.StopGlobe` (`self.LastBxVar`)))))

(event `FindPendant`
  ;[1 1 1] 펜던트 찾기
)

(event `self.ReceiveTick`
  (params (DeltaSeconds :type "Float (single-precision)"))
  ;[1 1 1] 펜던트 찾기
  (for _array_element (`PrimitiveComponent.GetOverlappingComponents` (`self.CompassCollision`))
    (if (`KismetStringLibrary.EqualEqual_StrStr` (`KismetSystemLibrary.GetObjectName` _array_element) "PendantCollision")
      (`KismetSystemLibrary.PrintString` "Collison OK"))))

(fn `ItemUsingPoint`
  (params (ItemID :type Integer))
  (returns (ItsUsed :type Boolean))
  (bind _returnvalue (== ItemID (`self.NeedItemID`)))
  (set `self.isItemUsed` _returnvalue)
  (`self.CompassAnimStart`)
  (return _returnvalue))

(fn `UserConstructionScript`)