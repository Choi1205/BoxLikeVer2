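; Inner puzzle box actor that the player manipulates by mouse-dragging its parts through a staged sequence.
; BlockMoving hands input from the player to the box until left mouse release.
; Boolean flags chain the stages: green button opens a piece, CD wheels enable the hexagon, which shifts the box and, if the BP_ItemKey is active, advances it and arms the side button.
; That button unlocks linked side drawers, one sliding while the other rotates.
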(event `self.ReceiveBeginPlay`
  (bind _outactors (`GameplayStatics.GetAllActorsOfClass` "/Game/BoxesLike/BluePrints/RealBoxYuchin/BP_ItemKey.BP_ItemKey_C"))
  (set `self.KeyVar` (`|GetArrayItem` _outactors)))

(event `/Game/BoxesLike/BPInterface/BlockMoving.Block Moving`
  (params (Mover :type "Pawn Object Reference") (ClickPoint :type "Vector Structure") (LookingComponentPoint :type "PrimitiveComponent Object Reference"))
  (bind _returnvalue (`GameplayStatics.GetPlayerController` 0))
  ;[1 1 1] 아이템 상세 확인 시작/종료 부분. 상세 확인을 시작하면 플레이어 캐릭터에 있던 컨트롤을 생성된 이 액터로 옮긴다.
  (if (or (== LookingComponentPoint (`self.GreenButton`)) (== LookingComponentPoint (`self.LeftCD`)) (== LookingComponentPoint (`self.RightCD`)) (== LookingComponentPoint (`self.Hexagon`)) (== LookingComponentPoint (`self.SideButton`)) (== LookingComponentPoint (`self.SideDowndrawer`)))
    (set `self.Looking Component Point` LookingComponentPoint)
    (`self.DisableInput` Mover _returnvalue)
    (`self.EnableInput` _returnvalue)))

(event `Key|LeftMouseButton`
  (params (Key :type "Key Structure"))
  (bind _returnvalue (`GameplayStatics.GetPlayerController` 0))
  (:`Released`
    (`self.DisableInput` _returnvalue)
    (`self.EnableInput` (stale `/Game/BoxesLike/BPInterface/BlockMoving.Block Moving` Mover) _returnvalue)))

(event `InputAxisKey|MouseX`
  (params (AxisValue :type "Float (single-precision)"))
  (bind (_relativelocation_x _relativelocation_y) (`KismetMathLibrary.BreakVector` (`SceneComponent.RelativeLocation` (`self.Hexagon`))))
  (bind (_relativelocation_x_2 _relativelocation_y_2) (`KismetMathLibrary.BreakVector` (`SceneComponent.RelativeLocation` (`self.GreenButton`))))
  (bind (_relativelocation_x_3 _relativelocation_y_3) (`KismetMathLibrary.BreakVector` (`SceneComponent.RelativeLocation` (`self.SideButton`))))
  (bind (_relativelocation_x_4 _relativelocation_y_4 _relativelocation_z) (`KismetMathLibrary.BreakVector` (`SceneComponent.RelativeLocation` (`self.Looking Component Point`))))
  (bind _returnvalue (+ _relativelocation_y_4 (* AxisValue 0.25)))
  ;[1 1 1] 마우스를 드래그하면 초록 버튼, Hexagon, Side Button y축(->)이동
  (if (`PlayerController.IsInputKeyDown` (`GameplayStatics.GetPlayerController` 0) "LeftMouseButton")
    (if (or (and (<= _returnvalue 7.0) (>= _returnvalue 4.5) (`self.isButtonAct`) (== (`self.Looking Component Point`) (`self.GreenButton`))) (and (<= _returnvalue 1.5) (>= _returnvalue -1.18) (`self.isHexagonAct`) (== (`self.Looking Component Point`) (`self.Hexagon`))) (and (<= _returnvalue -3.5) (>= _returnvalue -5.1) (`self.isSideBtAct`) (== (`self.Looking Component Point`) (`self.SideButton`))))
      (`SceneComponent.K2_SetRelativeLocation` (`self.Looking Component Point`) (`KismetMathLibrary.MakeVector` _relativelocation_x_4 _returnvalue _relativelocation_z) false false)
      (if (and (>= _relativelocation_y_2 6.8) (`self.isButtonAct`))
        (`KismetSystemLibrary.Delay` 0.2)
        (bind (_direction _btafteropen) (`Timeline|Timeline`)
          (:`Update`
            (`SceneComponent.K2_SetRelativeRotation` (`self.Open`) (`KismetMathLibrary.MakeRotator` 0.0 _btafteropen) false false)
            (set `self.isButtonAct` false)
            (set `self.isWheelAct` true)))
        (elif (and (>= _relativelocation_y 1.45) (`self.isHexagonAct`))
          (bind (_direction_2 _hexaafterboxmove) (`Timeline|Timeline_0`)
            (:`Update`
              (`SceneComponent.K2_SetRelativeLocation` (`self.MainBox`) (`KismetMathLibrary.MakeVector` _hexaafterboxmove) false false)
              (set `self.isHexagonAct` false)
              (if (`/Game/BoxesLike/BluePrints/RealBoxYuchin/BP_ItemKey.isItemAct` (`self.KeyVar`))
                (`/Game/BoxesLike/BluePrints/RealBoxYuchin/BP_ItemKey.ItemGoForward` (`self.KeyVar`))
                (set `self.isSideBtAct` true))))
          (elif (and (>= _relativelocation_y_3 -3.6) (`self.isSideBtAct`))
            (set `self.isSideBtAct` false)
            (set `self.isSideDownDwAct` true)
            (`KismetSystemLibrary.PrintString` "sdd ready")))))))

(event `InputAxisKey|MouseY`
  (params (AxisValue :type "Float (single-precision)"))
  (bind _returnvalue (* AxisValue (`self.dir`)))
  (bind (_relativelocation_x _relativelocation_y _relativelocation_z) (`KismetMathLibrary.BreakVector` (`SceneComponent.RelativeLocation` (`self.Looking Component Point`))))
  (bind _relativerotation_roll (`KismetMathLibrary.BreakRotator` (`SceneComponent.RelativeRotation` (`self.Looking Component Point`))))
  (bind (_relativerotation_roll_2 _relativerotation_pitch _relativerotation_yaw) (`KismetMathLibrary.BreakRotator` (`SceneComponent.RelativeRotation` (`self.Looking Component Point`))))
  (bind _relativerotation_roll_3 (`KismetMathLibrary.BreakRotator` (`SceneComponent.RelativeRotation` (`self.LeftCD`))))
  (bind _relativerotation_roll_4 (`KismetMathLibrary.BreakRotator` (`SceneComponent.RelativeRotation` (`self.RightCD`))))
  (bind (_relativelocation_x_2 _relativelocation_y_2 _relativelocation_z_2) (`KismetMathLibrary.BreakVector` (`SceneComponent.RelativeLocation` (`self.SideDowndrawer`))))
  (bind (_relativerotation_roll_5 _relativerotation_pitch_2 _relativerotation_yaw_2) (`KismetMathLibrary.BreakRotator` (`SceneComponent.RelativeRotation` (`self.SideUpdrawer`))))
  ;[1 1 1] CD 2개 회전
  (if (`PlayerController.IsInputKeyDown` (`GameplayStatics.GetPlayerController` 0) "LeftMouseButton")
    (if (and (or (>= _relativerotation_roll 0.5) (<= _relativerotation_roll -0.5)) (`self.isWheelAct`) (or (== (`self.Looking Component Point`) (`self.LeftCD`)) (== (`self.Looking Component Point`) (`self.RightCD`))))
      (`SceneComponent.K2_SetRelativeRotation` (`self.Looking Component Point`) (`KismetMathLibrary.MakeRotator` (+ _relativerotation_roll_2 _returnvalue) _relativerotation_pitch _relativerotation_yaw) false false)
      (if (and (or (>= _relativerotation_roll_3 -0.5) (<= _relativerotation_roll_3 0.5)) (or (>= _relativerotation_roll_4 -0.5) (<= _relativerotation_roll_4 0.5)))
        (set `self.isHexagonAct` true))
      (elif (and (== (`self.Looking Component Point`) (`self.SideDowndrawer`)) (`self.isSideDownDwAct`) (>= _returnvalue -4.0) (<= _returnvalue 0.6))
        (`KismetSystemLibrary.PrintString` (`KismetStringLibrary.Conv_DoubleToString` _returnvalue))
        (`SceneComponent.K2_SetRelativeLocation` (`self.Looking Component Point`) (`KismetMathLibrary.MakeVector` _relativelocation_x _relativelocation_y (+ _relativelocation_z (* _returnvalue -0.25))) false false)
        (`SceneComponent.K2_SetRelativeRotation` (`self.SideUpdrawer`) (`KismetMathLibrary.MakeRotator` _relativerotation_roll_5 (+ (* _returnvalue -5.0) _relativerotation_pitch_2) _relativerotation_yaw_2) false false)
        (if (>= _relativelocation_z_2 0.5)
          (set `self.isSideDownDwAct` false))))))

(fn `UserConstructionScript`)