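; BP_SecondBox is a box actor with two doors that open on an event or slide by mouse drag.
; DoorOpen plays a timeline that moves both doors in mirrored X directions.
; BlockMoving hands input from the player to the box when the looked-at component is a door.
; While left mouse is held, horizontal movement slides that door within its own X limits, and release returns control to the player.
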(event `DoorOpen`
  (bind (_direction _ldo) (`Timeline|LeftDoorOpen`)
    (:`Update`
      (`SceneComponent.K2_SetRelativeLocation` (`self.LeftDoor`) (`KismetMathLibrary.MakeVector` _ldo) false false)
      (`SceneComponent.K2_SetRelativeLocation` (`self.RightDoor`) (`KismetMathLibrary.MakeVector` (* _ldo -1.0)) false false))))

(event `/Game/BoxesLike/BPInterface/BlockMoving.Block Moving`
  (params (Mover :type "Pawn Object Reference") (ClickPoint :type "Vector Structure") (LookingComponentPoint :type "PrimitiveComponent Object Reference"))
  (bind _returnvalue (`GameplayStatics.GetPlayerController` 0))
  ;[1 1 1] 플레이어 캐릭터에 있던 컨트롤을 생성된 이 액터로 옮긴다.
  (if (or (== LookingComponentPoint (`self.LeftDoor`)) (== LookingComponentPoint (`self.RightDoor`)))
    (set `self.LookingComponentPoint` LookingComponentPoint)
    (`self.DisableInput` Mover _returnvalue)
    (`self.EnableInput` _returnvalue)))

(event `Key|LeftMouseButton`
  (params (Key :type "Key Structure"))
  (bind _returnvalue (`GameplayStatics.GetPlayerController` 0))
  ;[1 1 1] 플레이어 캐릭터에 있던 컨트롤을 생성된 이 액터로 옮긴다.
  (:`Released`
    (`self.DisableInput` _returnvalue)
    (`self.EnableInput` (stale `/Game/BoxesLike/BPInterface/BlockMoving.Block Moving` Mover) _returnvalue)))

(event `InputAxisKey|MouseX`
  (params (AxisValue :type "Float (single-precision)"))
  (bind (_relativelocation_x _relativelocation_y _relativelocation_z) (`KismetMathLibrary.BreakVector` (`SceneComponent.RelativeLocation` (`self.LookingComponentPoint`))))
  (bind _returnvalue (+ _relativelocation_x (* AxisValue -1.0)))
  (if (`PlayerController.IsInputKeyDown` (`GameplayStatics.GetPlayerController` 0) "LeftMouseButton")
    (if (and (<= _returnvalue 29.0) (>= _returnvalue 12.0) (== (`self.LookingComponentPoint`) (`self.LeftDoor`)))
      (`SceneComponent.K2_SetRelativeLocation` (`self.LookingComponentPoint`) (`KismetMathLibrary.MakeVector` _returnvalue _relativelocation_y _relativelocation_z) false false :!label _label)
      (elif (and (<= _returnvalue -12.0) (>= _returnvalue -30.0) (== (`self.LookingComponentPoint`) (`self.RightDoor`)))
        (goto _label)))))

(fn `UserConstructionScript`)