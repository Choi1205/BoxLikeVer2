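; BP_ItemShip is a collectible ship item that stays hidden and non-collidable until it is revealed.
; ShipForward enables the Ship component's visibility and collision, then plays a timeline that drives its relative X location.
; GetItem calls DestroyItem and returns the item's ID, name, texture and static mesh.
; DestroyItem delays briefly before destroying the actor so the return values arrive first, leaving room for an acquire animation.
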(event `self.ReceiveBeginPlay`
  (`SceneComponent.SetVisibility` (`self.Ship`) false false)
  (`PrimitiveComponent.SetCollisionEnabled` (`self.Ship`) "NoCollision"))

(event `ShipForward`
  (`PrimitiveComponent.SetCollisionEnabled` (`self.Ship`) "QueryAndPhysics")
  (`SceneComponent.SetVisibility` (`self.Ship`) true false)
  (bind (_direction _ship) (`Timeline|Timeline`)
    (:`Update`
      (`SceneComponent.K2_SetRelativeLocation` (`self.Ship`) (`KismetMathLibrary.MakeVector` _ship) false false))))

(event `Destroy Item`
  ;[1 1 1] 아이템 획득시 딜레이를 줘서 액터 삭제 전 리턴값을 줄 시간을 얻음.
  ; 액터 삭제 전 획득 애니메이션 삽입 가능
  (`KismetSystemLibrary.Delay` 0.2)
  (`KismetSystemLibrary.PrintString` "Shi[p Acquired")
  (`self.K2_DestroyActor`))

(fn `GetItem`
  (returns (ItemID :type Integer) (ItemName :type String) (ItemTexture :type "Texture2D Object Reference") (ItemStaticMesh :type "StaticMesh Object Reference"))
  (`self.Destroy Item`)
  (return (`self.ItemId`) (`self.ItemName`) (`self.ItemTexture`) (`self.ItemStaticmesh`)))

(fn `UserConstructionScript`)