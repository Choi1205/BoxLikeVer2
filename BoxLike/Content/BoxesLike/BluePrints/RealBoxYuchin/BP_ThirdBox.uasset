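; BP_ThirdBox is a puzzle box actor with a rotatable black outer circle and an animated metal sphere.
; BlockMoving hands input from the Mover to the box when the circle is targeted; releasing left mouse returns it.
; Held-mouse vertical movement rolls the circle and slightly pitches the inner glass sphere.
; ItemUsingPoint, without checking the item ID, reveals the metal sphere and plays its timeline-driven fall.
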(event `self.ReceiveBeginPlay`
  (`SceneComponent.SetVisibility` (`self.MetalSphereAnim`) false false))

(event `/Game/BoxesLike/BPInterface/BlockMoving.Block Moving`
  (params (Mover :type "Pawn Object Reference") (ClickPoint :type "Vector Structure") (LookingComponentPoint :type "PrimitiveComponent Object Reference"))
  (bind _returnvalue (`GameplayStatics.GetPlayerController` 0))
  ;[1 1 1] 플레이어 캐릭터에 있던 컨트롤을 생성된 이 액터로 옮긴다.
  (if (== LookingComponentPoint (`self.OutsideCircleBlack`))
    (set `self.LookingComponentPoint` LookingComponentPoint)
    (`self.DisableInput` Mover _returnvalue)
    (`self.EnableInput` _returnvalue)))

(event `Key|LeftMouseButton`
  (params (Key :type "Key Structure"))
  (bind _returnvalue (`GameplayStatics.GetPlayerController` 0))
  ;[1 1 1] 플레이어 캐릭터에 있던 컨트롤을 생성된 이 액터로 옮긴다.
  (:`Released`
    (`self.DisableInput` _returnvalue)
    (`self.EnableInput` (stale `/Game/BoxesLike/BPInterface/BlockMoving.Block Moving` Mover) _returnvalue)))

(event `MsAnimStart`
  (`SceneComponent.SetVisibility` (`self.MetalSphereAnim`) true false)
  (bind (_direction _msfall) (`Timeline|Timeline`)
    (:`Update`
      (`SceneComponent.K2_SetRelativeLocation` (`self.MetalSphereAnim`) (`KismetMathLibrary.MakeVector` 0.0 0.0 _msfall) false false))))

(event `InputAxisKey|MouseY`
  (params (AxisValue :type "Float (single-precision)"))
  (bind _returnvalue (* AxisValue -1.0))
  (bind _lookingcomponentpoint (`self.LookingComponentPoint`))
  (bind (_relativerotation_roll _relativerotation_pitch) (`KismetMathLibrary.BreakRotator` (`SceneComponent.RelativeRotation` (`self.GlassInsideSphere`))))
  (bind _relativerotation_roll_2 (`KismetMathLibrary.BreakRotator` (`SceneComponent.RelativeRotation` (`self.LookingComponentPoint`))))
  (bind (_relativerotation_roll_3 _relativerotation_pitch_2 _relativerotation_yaw) (`KismetMathLibrary.BreakRotator` (`SceneComponent.RelativeRotation` _lookingcomponentpoint)))
  (if (`PlayerController.IsInputKeyDown` (`GameplayStatics.GetPlayerController` 0) "LeftMouseButton")
    (if (== (`self.LookingComponentPoint`) (`self.OutsideCircleBlack`))
      (`SceneComponent.K2_SetRelativeRotation` _lookingcomponentpoint (`KismetMathLibrary.MakeRotator` (+ _relativerotation_roll_3 _returnvalue) _relativerotation_pitch_2 _relativerotation_yaw) false false)
      (`KismetSystemLibrary.PrintString` (`KismetStringLibrary.Conv_RotatorToString` (`SceneComponent.RelativeRotation` (`self.LookingComponentPoint`))))
      (`SceneComponent.K2_SetRelativeRotation` (`self.GlassInsideSphere`) (`KismetMathLibrary.MakeRotator` 0.0 (+ (* _returnvalue 0.0025) _relativerotation_pitch)) false false)
      (if (or (>= _relativerotation_roll_2 -179.5) (<= _relativerotation_roll_2 179.5))
        (set `self.isSphereAct` false)))))

(fn `ItemUsingPoint`
  (params (ItemID :type Integer))
  (returns (ItsUsed :type Boolean))
  (set `self.isItemUsed` false)
  (`self.MsAnimStart`)
  (return false))

(fn `UserConstructionScript`)