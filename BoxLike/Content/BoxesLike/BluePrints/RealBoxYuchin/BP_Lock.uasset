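; BP_Lock is an interactive puzzle lock that the player turns with a key to open the BP_SecondBox door.
; ItemUsingPoint compares the item ID with NeedItemID and, regardless of the result, starts a timeline that reveals and slides the key.
; BlockMoving takes input from the player, so left-mouse drag rolls the key until release.
; Near a half turn, the key hides, the lock falls and the box's DoorOpen runs after a delay.
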(event `self.ReceiveBeginPlay`
  (`SceneComponent.SetVisibility` (`self.keyAnim`) false false)
  (bind _outactors (`GameplayStatics.GetAllActorsOfClass` "/Game/BoxesLike/BluePrints/RealBoxYuchin/BP_SecondBox.BP_SecondBox_C"))
  (set `self.SecBoxVar` (`|GetArrayItem` _outactors)))

(event `/Game/BoxesLike/BPInterface/BlockMoving.Block Moving`
  (params (Mover :type "Pawn Object Reference") (ClickPoint :type "Vector Structure") (LookingComponentPoint :type "PrimitiveComponent Object Reference"))
  (bind _returnvalue (`GameplayStatics.GetPlayerController` 0))
  ;[1 1 1] 플레이어 캐릭터에 있던 컨트롤을 생성된 이 액터로 옮긴다.
  (if (== LookingComponentPoint (`self.keyAnim`))
    (set `self.Looking Component Point` LookingComponentPoint)
    (`self.DisableInput` Mover _returnvalue)
    (`self.EnableInput` _returnvalue)))

(event `Key|LeftMouseButton`
  (params (Key :type "Key Structure"))
  (bind _returnvalue (`GameplayStatics.GetPlayerController` 0))
  ;[1 1 1] 플레이어 캐릭터에 있던 컨트롤을 생성된 이 액터로 옮긴다.
  (:`Released`
    (`self.DisableInput` _returnvalue)
    (`self.EnableInput` (stale `/Game/BoxesLike/BPInterface/BlockMoving.Block Moving` Mover) _returnvalue)))

(event `KeyAnimStart`
  (`SceneComponent.SetVisibility` (`self.keyAnim`) true false)
  (bind (_direction _keygoforward) (`Timeline|Key`)
    (:`Update`
      (`SceneComponent.K2_SetRelativeLocation` (`self.keyAnim`) (`KismetMathLibrary.MakeVector` 0.0 _keygoforward) false false))))

(event `InputAxisKey|MouseY`
  (params (AxisValue :type "Float (single-precision)"))
  (bind _looking_component_point (`self.Looking Component Point`))
  (bind _relativerotation_roll (`KismetMathLibrary.BreakRotator` (`SceneComponent.RelativeRotation` (`self.Looking Component Point`))))
  (bind (_relativerotation_roll_2 _relativerotation_pitch _relativerotation_yaw) (`KismetMathLibrary.BreakRotator` (`SceneComponent.RelativeRotation` _looking_component_point)))
  (bind _relativerotation_roll_3 (`KismetMathLibrary.BreakRotator` (`SceneComponent.RelativeRotation` (`self.Looking Component Point`))))
  (if (`PlayerController.IsInputKeyDown` (`GameplayStatics.GetPlayerController` 0) "LeftMouseButton")
    (if (and (or (>= _relativerotation_roll_3 -179.5) (<= _relativerotation_roll_3 179.5)) (`self.isKeyAct`))
      (`SceneComponent.K2_SetRelativeRotation` _looking_component_point (`KismetMathLibrary.MakeRotator` (+ _relativerotation_roll_2 (* AxisValue -1.0)) _relativerotation_pitch _relativerotation_yaw) false false)
      (if (or (>= _relativerotation_roll 179.5) (<= _relativerotation_roll -179.5))
        (set `self.isKeyAct` false)
        (`SceneComponent.SetVisibility` (`self.keyAnim`) false false)
        (bind (_direction _fall) (`Timeline|LockFall`)
          (:`Update`
            (`SceneComponent.K2_SetRelativeLocation` (`self.Lock`) (`KismetMathLibrary.MakeVector` 0.0 0.0 _fall) false false)
            (`KismetSystemLibrary.Delay` 0.2)
            (`/Game/BoxesLike/BluePrints/RealBoxYuchin/BP_SecondBox.DoorOpen` (`self.SecBoxVar`))))))))

(fn `ItemUsingPoint`
  (params (ItemID :type Integer))
  (returns (ItsUsed :type Boolean))
  (bind _returnvalue (== ItemID (`self.NeedItemID`)))
  ;[1 1 1] It's SAME 위치에 키 작용 애니메이션을 넣을 것
  (set `self.isItemUsed` _returnvalue)
  (`self.KeyAnimStart`)
  (return _returnvalue))

(fn `UserConstructionScript`)