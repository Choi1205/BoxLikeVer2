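; BP_ThirdBox is an interactive puzzle box where rotating a dial turns a glass sphere to bring a metal ball to a target.
; Using an item reveals and drops the ball via timeline, regardless of ID match.
; Targeting OutsideCircleBlack shifts input from Mover to the box for mouse-drag rotation until release.
; Overlapping SphereDestin ends rotation, swaps decorations for lights after a delay, then later calls Lighting on BP_FourthBox.
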(event `self.ReceiveBeginPlay`
  (`SceneComponent.SetVisibility` (`self.MetalSphereAnim`) false false)
  (`SceneComponent.SetVisibility` (`self.Light2-4`) false false)
  (`SceneComponent.SetVisibility` (`self.Light2-1`) false false)
  (`SceneComponent.SetVisibility` (`self.Light2-2`) false false)
  (`SceneComponent.SetVisibility` (`self.Light2-3`) false false)
  (bind _outactors (`GameplayStatics.GetAllActorsOfClass` "/Game/BoxesLike/BluePrints/RealBoxYuchin/BP_FourthBox.BP_FourthBox_C"))
  (set `self.FB_Var` (`|GetArrayItem` _outactors)))

(event `/Game/BoxesLike/BPInterface/BlockMoving.Block Moving`
  (params (Mover :type "Pawn Object Reference") (ClickPoint :type "Vector Structure") (LookingComponentPoint :type "PrimitiveComponent Object Reference"))
  (bind _returnvalue (`GameplayStatics.GetPlayerController` 0))
  ;[1 1 1] 플레이어 캐릭터에 있던 컨트롤을 생성된 이 액터로 옮긴다.
  (if (== LookingComponentPoint (`self.OutsideCircleBlack`))
    (set `self.LookingComponentPoint` LookingComponentPoint)
    (`self.DisableInput` Mover _returnvalue)
    (`self.EnableInput` _returnvalue)))

(event `Key|LeftMouseButton`
  (params (Key :type "Key Structure"))
  (bind _returnvalue (`GameplayStatics.GetPlayerController` 0))
  ;[1 1 1] 플레이어 캐릭터에 있던 컨트롤을 생성된 이 액터로 옮긴다.
  (:`Released`
    (`self.DisableInput` _returnvalue)
    (`self.EnableInput` (stale `/Game/BoxesLike/BPInterface/BlockMoving.Block Moving` Mover) _returnvalue)))

(event `MsAnimStart`
  (`SceneComponent.SetVisibility` (`self.MetalSphereAnim`) true false)
  (bind (_direction _msfall) (`Timeline|Timeline`)
    (:`Update`
      (`SceneComponent.K2_SetRelativeLocation` (`self.MetalSphereAnim`) (`KismetMathLibrary.MakeVector` 0.0 0.0 _msfall) false false))))

(event `InputAxisKey|MouseY`
  (params (AxisValue :type "Float (single-precision)"))
  (bind _returnvalue (* AxisValue -1.0))
  (bind _lookingcomponentpoint (`self.LookingComponentPoint`))
  (bind (_relativerotation_roll _relativerotation_pitch _relativerotation_yaw) (`KismetMathLibrary.BreakRotator` (`SceneComponent.RelativeRotation` _lookingcomponentpoint)))
  (if (`PlayerController.IsInputKeyDown` (`GameplayStatics.GetPlayerController` 0) "LeftMouseButton")
    (if (and (`self.isSphereAct`) (== (`self.LookingComponentPoint`) (`self.OutsideCircleBlack`)))
      (`SceneComponent.K2_SetRelativeRotation` _lookingcomponentpoint (`KismetMathLibrary.MakeRotator` (+ _relativerotation_roll _returnvalue) _relativerotation_pitch _relativerotation_yaw) false false) ; 초록 버튼을 회진시키면
      (`SceneComponent.K2_AddLocalRotation` (`self.GlassInsideSphere`) (`KismetMathLibrary.MakeRotator` 0.0 (* _returnvalue 0.5)) false false) ; GlassInsideSphere도 회전함
      (if (`PrimitiveComponent.IsOverlappingComponent` (`self.MetalSphereAnim`) (`self.SphereDestin`))
        (set `self.isSphereAct` false)
        (`KismetSystemLibrary.Delay` 3.0)
        (`SceneComponent.SetVisibility` (`self.Deco2-4`) false false)
        (`SceneComponent.SetVisibility` (`self.Deco2-1`) false false)
        (`SceneComponent.SetVisibility` (`self.Deco2-2`) false false)
        (`SceneComponent.SetVisibility` (`self.Deco2-3`) false false)
        (`SceneComponent.SetVisibility` (`self.Light2-4`) true false)
        (`SceneComponent.SetVisibility` (`self.Light2-1`) true false)
        (`SceneComponent.SetVisibility` (`self.Light2-2`) true false)
        (`SceneComponent.SetVisibility` (`self.Light2-3`) true false)
        (if (not (`self.isSphereAct`))
          (`KismetSystemLibrary.Delay` 10.0)
          (`/Game/BoxesLike/BluePrints/RealBoxYuchin/BP_FourthBox.Lighting` (`self.FB_Var`)))))))

(fn `ItemUsingPoint`
  (params (ItemID :type Integer))
  (returns (ItsUsed :type Boolean))
  (bind _returnvalue (== ItemID (`self.NeedItemID`)))
  (set `self.isItemUsed` _returnvalue)
  (`self.MsAnimStart`)
  (return _returnvalue))

(fn `UserConstructionScript`)