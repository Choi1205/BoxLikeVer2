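; BP_Door is a click-driven rotating door puzzle piece that turns its ShapePieces component in quarter-turn steps.
; Clicking Button cyclically shifts the first four OutsideArr entries through swaps, prints the new first entry, then plays the Rotate90 timeline to lerp the yaw with a negated alpha.
; A counter caps the rotations but not the array shift, and IsRotate is set when each turn finishes.
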(event `self.ReceiveBeginPlay`
  (set `PlayerController.bEnableClickEvents` true (`GameplayStatics.GetPlayerController` 0)))

(event `self.Button.OnClicked`
  (params (TouchedComponent :type "PrimitiveComponent Object Reference") (ButtonPressed :type "Key Structure"))
  (bind _outsidearr (`self.outsideArr`))
  (`KismetArrayLibrary.Array_Swap` _outsidearr 0 1)
  (`KismetArrayLibrary.Array_Swap` _outsidearr 1 2)
  (`KismetArrayLibrary.Array_Swap` _outsidearr 2 3)
  (`KismetSystemLibrary.PrintString` (`KismetStringLibrary.Conv_IntToString` (`|GetArrayItem` _outsidearr)))
  (bind _output_get (set `self.startRotation` (`SceneComponent.RelativeRotation` (`self.ShapePieces`))))
  (set `self.endRotation` (`KismetMathLibrary.ComposeRotators` _output_get (struct :`Pitch` 90.0)))
  (if (<= (`self.cnt`) 10)
    (bind (_direction _rotate) (`Timeline|Rotate90` :!via `PlayFromStart`)
      (:`Update`
        (`SceneComponent.K2_SetRelativeRotation` (`self.ShapePieces`) (`KismetMathLibrary.RLerp` (`self.startRotation`) (`self.endRotation`) (* _rotate -1.0) true) false false))
      (:`Finished`
        (set `self.cnt` (+ (`self.cnt`) 1))
        (set `self.isRotate` true)))))

(fn `UserConstructionScript`)