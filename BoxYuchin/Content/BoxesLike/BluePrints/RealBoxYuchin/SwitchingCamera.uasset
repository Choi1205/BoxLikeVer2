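; SwitchingCamera is an actor that switches the player's view to an alternate camera, apparently for a door, and back to the character.
; SwitchCamera spawns a BP_CameraActor at the SwitchedCamera component's relative transform, attaches it with relative rules, then makes it the view target.
; Back returns the view to the player character; both events update IsSwitchCamera and print debug text.
; Each switch spawns a new camera, and none is destroyed here.
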(event `SwitchCamera`
  (bind _returnvalue (`|SpawnActorFromClass` "/Game/BoxesLike/BluePrints/TestBoxBP/BP_CameraActor.BP_CameraActor_C" (`SceneComponent.GetRelativeTransform` (`self.SwitchedCamera`)) "Undefined" "MultiplyWithRoot" null null))
  (`self.K2_AttachToActor` _returnvalue self "None" "KeepRelative" "KeepRelative" "KeepRelative" true)
  (bind _output_get (set `self.CameraActor` _returnvalue))
  (`PlayerController.SetViewTargetWithBlend` (`GameplayStatics.GetPlayerController` 0) _output_get 0.0 "VTBlend_Linear" 0.0 false)
  (set `self.isSwitchCamera` true)
  (`KismetSystemLibrary.PrintString` "switch to door"))

(event `Back`
  (`PlayerController.SetViewTargetWithBlend` (`GameplayStatics.GetPlayerController` 0) (`GameplayStatics.GetPlayerCharacter` 0) 0.0 "VTBlend_Linear" 0.0 false)
  (set `self.isSwitchCamera` false)
  (`KismetSystemLibrary.PrintString` "door to character"))

(fn `UserConstructionScript`)