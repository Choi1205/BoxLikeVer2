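; BP_LastBoxGlobe is a globe actor that the player rotates by dragging with the left mouse button.
; BlockMoving hands input from the Mover to this actor when the looked-at component is the Globe; releasing the button hands it back.
; Mouse X drives local yaw and Mouse Y local pitch, only while IsGlobeAct is true.
; StopGlobe, noted as triggered by placing the Compass, halts RotatingMovement and sets that flag after a short delay.
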(event `self.ReceiveBeginPlay`)

(event `/Game/BoxesLike/BPInterface/BlockMoving.Block Moving`
  (params (Mover :type "Pawn Object Reference") (ClickPoint :type "Vector Structure") (LookingComponentPoint :type "PrimitiveComponent Object Reference"))
  (bind _returnvalue (`GameplayStatics.GetPlayerController` 0))
  ;[1 1 1] 플레이어 캐릭터에 있던 컨트롤을 생성된 이 액터로 옮긴다.
  (if (== LookingComponentPoint (`self.Globe`))
    (set `self.LookingComponentPoint` LookingComponentPoint)
    (`self.DisableInput` Mover _returnvalue)
    (`self.EnableInput` _returnvalue)))

(event `Key|LeftMouseButton`
  (params (Key :type "Key Structure"))
  (bind _returnvalue (`GameplayStatics.GetPlayerController` 0))
  ;[1 1 1] 플레이어 캐릭터에 있던 컨트롤을 생성된 이 액터로 옮긴다.
  (:`Released`
    (`self.DisableInput` _returnvalue)
    (`self.EnableInput` (stale `/Game/BoxesLike/BPInterface/BlockMoving.Block Moving` Mover) _returnvalue)))

(event `StopGlobe`
  (`ActorComponent.Deactivate` (`self.RotatingMovement`)) ; Compass 놓으면 globe 회전 멈춤
  (`KismetSystemLibrary.Delay` 1.0)
  (set `self.isGlobeAct` true))

(event `InputAxisKey|MouseX`
  (params (AxisValue :type "Float (single-precision)"))
  ;[1 1 1] Globe z축 회전
  (if (`PlayerController.IsInputKeyDown` (`GameplayStatics.GetPlayerController` 0) "LeftMouseButton")
    (if (`self.isGlobeAct`)
      (`SceneComponent.K2_AddLocalRotation` (`self.LookingComponentPoint`) (`KismetMathLibrary.MakeRotator` 0.0 0.0 (* AxisValue -1.0)) false false))))

(event `InputAxisKey|MouseY`
  (params (AxisValue :type "Float (single-precision)"))
  ;[1 1 1] Globe y축 회전
  (if (`PlayerController.IsInputKeyDown` (`GameplayStatics.GetPlayerController` 0) "LeftMouseButton")
    (if (`self.isGlobeAct`)
      (`SceneComponent.K2_AddLocalRotation` (`self.LookingComponentPoint`) (`KismetMathLibrary.MakeRotator` 0.0 AxisValue) false false))))

(fn `UserConstructionScript`)