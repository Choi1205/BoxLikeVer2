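; Puzzle box Blueprint with two rotatable shells and a pair of doors, operated by mouse dragging.
; BlockMoving hands input from the Mover to this actor when a movable part is targeted; releasing left mouse returns it.
; MouseY rolls the targeted shell until the roll check passes, then a timeline swings both doors open and disables shell collision and rotation.
; MouseX then turns either opened door manually within yaw limits.
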(event `/Game/BoxesLike/BPInterface/BlockMoving.Block Moving`
  (params (Mover :type "Pawn Object Reference") (ClickPoint :type "Vector Structure") (LookingComponentPoint :type "PrimitiveComponent Object Reference"))
  (bind _returnvalue (`GameplayStatics.GetPlayerController` 0))
  ;[1 1 1] 플레이어 캐릭터에 있던 컨트롤을 생성된 이 액터로 옮긴다.
  (if (or (== LookingComponentPoint (`self.UpBase`)) (== LookingComponentPoint (`self.DownBase`)) (== LookingComponentPoint (`self.LeftOpen`)) (== LookingComponentPoint (`self.RightOpen`)))
    (set `self.LookingComponentPoint` LookingComponentPoint)
    (`self.DisableInput` Mover _returnvalue)
    (`self.EnableInput` _returnvalue)))

(event `Key|LeftMouseButton`
  (params (Key :type "Key Structure"))
  (bind _returnvalue (`GameplayStatics.GetPlayerController` 0))
  ;[1 1 1] 플레이어 캐릭터에 있던 컨트롤을 생성된 이 액터로 옮긴다.
  (:`Released`
    (`self.DisableInput` _returnvalue)
    (`self.EnableInput` (stale `/Game/BoxesLike/BPInterface/BlockMoving.Block Moving` Mover) _returnvalue)))

(event `InputAxisKey|MouseY`
  (params (AxisValue :type "Float (single-precision)"))
  (bind _relativerotation_roll (`KismetMathLibrary.BreakRotator` (`SceneComponent.RelativeRotation` (`self.DownBase`))))
  (bind _relativerotation_roll_2 (`KismetMathLibrary.BreakRotator` (`SceneComponent.RelativeRotation` (`self.UpBase`))))
  ;[1 1 1] 드래그로 돌려서 문 열기
  (set `self.AxisValueY` AxisValue)
  (if (`PlayerController.IsInputKeyDown` (`GameplayStatics.GetPlayerController` 0) "LeftMouseButton")
    (if (and (== (`self.LookingComponentPoint`) (`self.UpBase`)) (`self.isShellRotate`))
      (`GameplayStatics.PlaySound2D` "/Game/BoxesLike/Sound/SE/Yuchin/FourthB_4-1_ShellRotate_Cue.FourthB_4-1_ShellRotate_Cue" 1.0 1.0 0.0 null null)
      (`SceneComponent.K2_AddLocalRotation` (`self.UpBase`) (`KismetMathLibrary.MakeRotator` (* (`self.AxisValueY`) -1.0)) false false)
      (if (and (or (<= _relativerotation_roll_2 3.0) (>= _relativerotation_roll_2 -3.0)) (or (<= _relativerotation_roll -177.0) (>= _relativerotation_roll 177.0))) :!label _label
        (`GameplayStatics.PlaySound2D` "/Game/BoxesLike/Sound/SE/Yuchin/FourthB_4-1_ShellDoorAutoOpen_Cue.FourthB_4-1_ShellDoorAutoOpen_Cue" 1.0 1.0 0.0 null null)
        (bind (_direction _open) (`Timeline|Timeline`)
          (:`Update`
            (`SceneComponent.K2_SetRelativeRotation` (`self.LeftOpen`) (`KismetMathLibrary.MakeRotator` 0.0 0.0 _open) false false)
            (`SceneComponent.K2_SetRelativeRotation` (`self.RightOpen`) (`KismetMathLibrary.MakeRotator` 0.0 0.0 (* _open -1.0)) false false)
            (`PrimitiveComponent.SetCollisionEnabled` (`self.UpBase`) "NoCollision")
            (`PrimitiveComponent.SetCollisionEnabled` (`self.DownBase`) "NoCollision")
            (set `self.isShellRotate` false)
            (set `self.isOpen` true))))
      (elif (and (== (`self.LookingComponentPoint`) (`self.DownBase`)) (`self.isShellRotate`))
        (`GameplayStatics.PlaySound2D` "/Game/BoxesLike/Sound/SE/Yuchin/FourthB_4-1_ShellRotate_Cue.FourthB_4-1_ShellRotate_Cue" 1.0 1.0 0.0 null null)
        (`SceneComponent.K2_AddLocalRotation` (`self.DownBase`) (`KismetMathLibrary.MakeRotator` (`self.AxisValueY`)) false false)
        (goto _label)))))

(event `InputAxisKey|MouseX`
  (params (AxisValue :type "Float (single-precision)"))
  (bind (_relativerotation_roll _relativerotation_pitch _relativerotation_yaw) (`KismetMathLibrary.BreakRotator` (`SceneComponent.RelativeRotation` (`self.RightOpen`))))
  (bind (_relativerotation_roll_2 _relativerotation_pitch_2 _relativerotation_yaw_2) (`KismetMathLibrary.BreakRotator` (`SceneComponent.RelativeRotation` (`self.LeftOpen`))))
  ;[1 1 1] 메달 문 수동 open
  (set `self.AxisValueX` AxisValue)
  (if (`PlayerController.IsInputKeyDown` (`GameplayStatics.GetPlayerController` 0) "LeftMouseButton")
    (if (and (== (`self.LookingComponentPoint`) (`self.LeftOpen`)) (`self.isOpen`) (>= _relativerotation_yaw_2 100.0) (<= _relativerotation_yaw_2 210.0))
      (`SceneComponent.K2_AddLocalRotation` (`self.LeftOpen`) (`KismetMathLibrary.MakeRotator` 0.0 0.0 (* (`self.AxisValueX`) -1.0)) false false)
      (elif (and (== (`self.LookingComponentPoint`) (`self.RightOpen`)) (`self.isOpen`) (>= _relativerotation_yaw -210.0) (<= _relativerotation_yaw -90.0))
        (`SceneComponent.K2_AddLocalRotation` (`self.RightOpen`) (`KismetMathLibrary.MakeRotator` 0.0 0.0 (* (`self.AxisValueX`) -1.0)) false false)))))

(fn `UserConstructionScript`)