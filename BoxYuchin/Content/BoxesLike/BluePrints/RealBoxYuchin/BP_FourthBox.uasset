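; Puzzle box actor with two mouse-dragged wheels that open its doors once aligned.
; BlockMoving hands input from the Mover to the box until mouse release; vertical drag turns a wheel and LeftInteract or Middle.
; When both pitches sit in hardcoded windows, Update-chained timelines hide the wheels and swing the doors open.
; Lighting reveals hidden targets; Tick shows each light while its piece overlaps its target, independently of the solve check.
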(event `self.ReceiveBeginPlay`
  (`SceneComponent.SetVisibility` (`self.Target1`) false false)
  (`SceneComponent.SetVisibility` (`self.Target2`) false false)
  (`SceneComponent.SetVisibility` (`self.Target3`) false false)
  (`SceneComponent.SetVisibility` (`self.Target4`) false false)
  (`SceneComponent.SetVisibility` (`self.DifTarget`) false false)
  (`SceneComponent.SetVisibility` (`self.Light1`) false false)
  (`SceneComponent.SetVisibility` (`self.Light2`) false false)
  (`SceneComponent.SetVisibility` (`self.Light3`) false false)
  (`SceneComponent.SetVisibility` (`self.Light4`) false false)
  (`SceneComponent.SetVisibility` (`self.LightDiffT`) false false))

(event `/Game/BoxesLike/BPInterface/BlockMoving.Block Moving`
  (params (Mover :type "Pawn Object Reference") (ClickPoint :type "Vector Structure") (LookingComponentPoint :type "PrimitiveComponent Object Reference"))
  (bind _returnvalue (`GameplayStatics.GetPlayerController` 0))
  ;[1 1 1] 플레이어 캐릭터에 있던 컨트롤을 생성된 이 액터로 옮긴다.
  (if (or (== LookingComponentPoint (`self.LeftWheel`)) (== LookingComponentPoint (`self.RightWheel`)))
    (set `self.LookingComponentPoint` LookingComponentPoint)
    (`self.DisableInput` Mover _returnvalue)
    (`self.EnableInput` _returnvalue)))

(event `Key|LeftMouseButton`
  (params (Key :type "Key Structure"))
  (bind _returnvalue (`GameplayStatics.GetPlayerController` 0))
  ;[1 1 1] 플레이어 캐릭터에 있던 컨트롤을 생성된 이 액터로 옮긴다.
  (:`Released`
    (`self.DisableInput` _returnvalue)
    (`self.EnableInput` (stale `/Game/BoxesLike/BPInterface/BlockMoving.Block Moving` Mover) _returnvalue)))

(event `Lighting`
  (`SceneComponent.SetVisibility` (`self.Target1`) true false)
  (`SceneComponent.SetVisibility` (`self.Target2`) true false)
  (`SceneComponent.SetVisibility` (`self.Target3`) true false)
  (`SceneComponent.SetVisibility` (`self.Target4`) true false)
  (`SceneComponent.SetVisibility` (`self.DifTarget`) true false))

(event `InputAxisKey|MouseY`
  (params (AxisValue :type "Float (single-precision)"))
  (bind _returnvalue (* AxisValue -0.75))
  (bind _leftinteract (`self.LeftInteract`))
  (bind _middle (`self.Middle`))
  (bind (_relativerotation_roll _relativerotation_pitch) (`KismetMathLibrary.BreakRotator` (`SceneComponent.RelativeRotation` (`self.LeftInteract`))))
  (bind (_relativerotation_roll_2 _relativerotation_pitch_2 _relativerotation_yaw) (`KismetMathLibrary.BreakRotator` (`SceneComponent.RelativeRotation` (`self.RightWheel`))))
  (bind (_relativerotation_roll_3 _relativerotation_pitch_3 _relativerotation_yaw_2) (`KismetMathLibrary.BreakRotator` (`SceneComponent.RelativeRotation` (`self.LeftWheel`))))
  (bind (_relativerotation_roll_4 _relativerotation_pitch_4) (`KismetMathLibrary.BreakRotator` (`SceneComponent.RelativeRotation` (`self.Middle`))))
  ;[1 1 1] 물레방아 드래그 회전
  (if (`PlayerController.IsInputKeyDown` (`GameplayStatics.GetPlayerController` 0) "LeftMouseButton")
    (if (and (`self.isWheelAct`) (== (`self.LookingComponentPoint`) (`self.LeftWheel`)))
      (`SceneComponent.K2_SetRelativeRotation` (`self.LeftWheel`) (`KismetMathLibrary.MakeRotator` (+ _relativerotation_roll_3 _returnvalue) _relativerotation_pitch_3 _relativerotation_yaw_2) false false)
      (`SceneComponent.K2_AddLocalRotation` _leftinteract (`KismetMathLibrary.MakeRotator` 0.0 0.0 _returnvalue) false false)
      (`KismetSystemLibrary.PrintString` (`KismetStringLibrary.Conv_RotatorToString` (`SceneComponent.RelativeRotation` _leftinteract)))
      (if (and (and (>= _relativerotation_pitch 87.0) (<= _relativerotation_pitch 92.0)) (and (>= _relativerotation_pitch_4 -75.0) (<= _relativerotation_pitch_4 -70.0))) :!label _label
        (set `self.isWheelAct` false)
        (`KismetSystemLibrary.Delay` 1.0)
        (bind (_direction _lwh) (`Timeline|HideLW`)
          (:`Update`
            (`SceneComponent.K2_SetRelativeLocation` (`self.LeftWheel`) (`KismetMathLibrary.MakeVector` _lwh) false false)
            (bind (_direction_2 _rwh) (`Timeline|HideRW`)
              (:`Update`
                (`SceneComponent.K2_SetRelativeLocation` (`self.RightWheel`) (`KismetMathLibrary.MakeVector` _rwh) false false)
                (`KismetSystemLibrary.Delay` 1.0)
                (bind (_direction_3 _ldo4) (`Timeline|OpenLD`)
                  (:`Update`
                    (`SceneComponent.K2_SetRelativeRotation` (`self.LeftDoor`) (`KismetMathLibrary.MakeRotator` 0.0 0.0 _ldo4) false false)
                    (bind (_direction_4 _rdo4) (`Timeline|OpenRD`)
                      (:`Update`
                        (`SceneComponent.K2_SetRelativeRotation` (`self.RightDoor`) (`KismetMathLibrary.MakeRotator` 0.0 0.0 _rdo4) false false))))))))))
      (elif (and (`self.isWheelAct`) (== (`self.LookingComponentPoint`) (`self.RightWheel`)))
        (`SceneComponent.K2_SetRelativeRotation` (`self.RightWheel`) (`KismetMathLibrary.MakeRotator` (+ _returnvalue _relativerotation_roll_2) _relativerotation_pitch_2 _relativerotation_yaw) false false)
        (`SceneComponent.K2_AddLocalRotation` _middle (`KismetMathLibrary.MakeRotator` 0.0 0.0 _returnvalue) false false)
        (`KismetSystemLibrary.PrintString` (`KismetStringLibrary.Conv_RotatorToString` (`SceneComponent.RelativeRotation` _middle)))
        (goto _label)))))

(event `self.ReceiveTick`
  (params (DeltaSeconds :type "Float (single-precision)"))
  (bind _light1 (`self.Light1`))
  (bind _light2 (`self.Light2`))
  (bind _light3 (`self.Light3`))
  (bind _light4 (`self.Light4`))
  (bind _lightdifft (`self.LightDiffT`))
  (if (`PrimitiveComponent.IsOverlappingComponent` (`self.Circle1`) (`self.Target1`))
    (`SceneComponent.SetVisibility` _light1 true false)
    (`KismetSystemLibrary.PrintString` "yes")
    (else
      (`SceneComponent.SetVisibility` _light1 false false)
      (`KismetSystemLibrary.PrintString` "No")))
  (if (`PrimitiveComponent.IsOverlappingComponent` (`self.Circle2`) (`self.Target2`))
    (`SceneComponent.SetVisibility` _light2 true false)
    (else
      (`SceneComponent.SetVisibility` _light2 false false)))
  (if (`PrimitiveComponent.IsOverlappingComponent` (`self.Circle3`) (`self.Target3`))
    (`SceneComponent.SetVisibility` _light3 true false)
    (else
      (`SceneComponent.SetVisibility` _light3 false false)))
  (if (`PrimitiveComponent.IsOverlappingComponent` (`self.Circle4`) (`self.Target4`))
    (`SceneComponent.SetVisibility` _light4 true false)
    (else
      (`SceneComponent.SetVisibility` _light4 false false)))
  (if (`PrimitiveComponent.IsOverlappingComponent` (`self.Different`) (`self.DifTarget`))
    (`SceneComponent.SetVisibility` _lightdifft true false)
    (else
      (`SceneComponent.SetVisibility` _lightdifft false false))))

(fn `UserConstructionScript`)