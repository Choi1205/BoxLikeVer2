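; Inspectable pickup actor that hides a second item, collected by clicking a capsule hotspot on it.
; StartInspect moves input from the inspecting character to the actor, so left-drag rotates ItemBody and right-click returns control.
; Clicking the capsule, found by cursor trace, passes the inner item to BP_FirstPersonCharacter, clears its widget info and exits inspection.
; GetItem returns the item's own data, delaying destruction briefly so the return values survive.
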(event `DestoryItem`
  ;[1 1 1] 아이템 획득시 딜레이를 줘서 액터 삭제 전 리턴값을 줄 시간을 얻음.
  ; 액터 삭제 전 획득 애니메이션 삽입 가능
  (`KismetSystemLibrary.Delay` 0.2)
  (`self.K2_DestroyActor`))

(event `/Game/BoxesLike/BPInterface/StartInspect.StartInspect`
  (params (Inspector :type "Pawn Object Reference"))
  (bind _returnvalue (`GameplayStatics.GetPlayerController` 0))
  ;[1 1 1] 아이템 상세 확인 시작/종료 부분. 상세 확인을 시작하면 플레이어 캐릭터에 있던 컨트롤을 생성된 이 액터로 옮긴다.
  (bind _output_get (set `self.Inspector` Inspector))
  (`self.DisableInput` _output_get _returnvalue)
  (`self.EnableInput` _returnvalue))

(event `Key|RightMouseButton`
  (params (Key :type "Key Structure"))
  (bind _returnvalue (`GameplayStatics.GetPlayerController` 0))
  ;[1 1 1] 아이템 상세 확인 시작/종료 부분. 상세 확인을 시작하면 플레이어 캐릭터에 있던 컨트롤을 생성된 이 액터로 옮긴다.
  (:`Pressed`
    (`self.DisableInput` _returnvalue :!label _label)
    (`self.EnableInput` (`self.Inspector`) _returnvalue)
    (bind _asbp_first_person_character (cast `/Game/FirstPerson/Blueprints/BP_FirstPersonCharacter` (`GameplayStatics.GetPlayerCharacter` 0)))
    (`/Game/FirstPerson/Blueprints/BP_FirstPersonCharacter.EndInspectMouse` _asbp_first_person_character)))

(event `GetInsideItem`
  ;[1 1 1] 아이템 상세 확인 시작/종료 부분. 상세 확인을 시작하면 플레이어 캐릭터에 있던 컨트롤을 생성된 이 액터로 옮긴다.
  (goto _label))

(event `InputAxisKey|MouseX`
  (params (AxisValue :type "Float (single-precision)"))
  ;[1 1 1] 마우스를 드래그하면 이 스태틱 매쉬가 회전한다.
  (if (`PlayerController.IsInputKeyDown` (`GameplayStatics.GetPlayerController` 0) "LeftMouseButton")
    (`SceneComponent.K2_SetRelativeRotation` (`self.ItemBody`) (`KismetMathLibrary.ComposeRotators` (`self.K2_GetActorRotation`) (`KismetMathLibrary.MakeRotator` 0.0 0.0 (* AxisValue -1.0))) false false)))

(event `InputAxisKey|MouseY`
  (params (AxisValue :type "Float (single-precision)"))
  ;[1 1 1] 마우스를 드래그하면 이 스태틱 매쉬가 회전한다.
  (if (`PlayerController.IsInputKeyDown` (`GameplayStatics.GetPlayerController` 0) "LeftMouseButton")
    (`SceneComponent.K2_SetRelativeRotation` (`self.ItemBody`) (`KismetMathLibrary.ComposeRotators` (`self.K2_GetActorRotation`) (`KismetMathLibrary.MakeRotator` 0.0 (* AxisValue -1.0))) false false)))

(event `Key|LeftMouseButton`
  (params (Key :type "Key Structure"))
  ;[1 1 1] 아이템 안의 아이템을 획득했을때 사용.
  (:`Pressed`
    (if (== (`self.Capsule`) (`.HitComponent` (`GameplayStatics.BreakHitResult` (`PlayerController.GetHitResultUnderCursorForObjects` (`GameplayStatics.GetPlayerController` 0) (`|MakeArray` "ObjectTypeQuery2" :!type "EObjectTypeQuery Enum") true))))
      (bind _asbp_first_person_character (cast `/Game/FirstPerson/Blueprints/BP_FirstPersonCharacter` (`self.Inspector`)))
      (`/Game/FirstPerson/Blueprints/BP_FirstPersonCharacter.GetInsideItem` _asbp_first_person_character (`self.InsideItemID`) (`self.InsideItemName`) (`self.InsideItemTexture`) (`self.InsideItemStaticMesh`)) ; 내부 아이템 등록
      (`/Game/BoxesLike/BluePrints/UI_OnScreenWidget.DeleteInsideItemInfo` (`self.OnScreenWidget`) (`self.ItemID`)) ; 우측에 표시된 아이템 정보 삭제
      (`self.GetInsideItem`) ; 아이템을 획득하면 이 아이템의 조사모드 종료
    )))

(fn `GetItem`
  (returns (ItemID :type Integer) (ItemName :type String) (ItemTexture :type "Texture2D Object Reference") (ItemStaticMesh :type "StaticMesh Object Reference"))
  ;[1 1 1] 리턴값이 있으므로 딜레이를 줘서 값이 소실되는 것을 방지
  (`self.DestoryItem`)
  (return (`self.ItemID`) (`self.ItemName`) (`self.ItemTexture`) (`self.ItemStaticMesh`)))

(fn `UserConstructionScript`)