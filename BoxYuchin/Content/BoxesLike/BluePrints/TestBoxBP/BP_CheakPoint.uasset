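; BP_CheakPoint is an inspection point that smoothly zooms the player's view in on itself and later returns it to the character.
; On BeginPlay it spawns and attaches a camera actor using CameraMovingPosition's relative transform, because view-target blending needs an actor.
; ZoomIn blends to that camera, disables Cube collision to avoid blocking clicks and returns the zoomed actor.
; ReturnToPlayer blends back and restores collision.
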(event `self.ReceiveBeginPlay`
  ;[1 1 1] 게임이 시작되면 카메라 무빙 포지션 위치에 카메라 액터를 생성, 자식으로 붙여버린다.
  ; 카메라 컴포넌트에는 SetViewTargetwithBlend를 사용할 수 없어서 굳이 액터로 생성하고 있다.
  ; 카메라 컴포넌트는 뷰포트에서 배치할때 어떤 화면으로 보이는지 확인용.
  (bind _returnvalue (`|SpawnActorFromClass` "/Game/BoxesLike/BluePrints/TestBoxBP/BP_CameraActor.BP_CameraActor_C" (`SceneComponent.GetRelativeTransform` (`self.CameraMovingPosition`)) "Undefined" "MultiplyWithRoot" null null))
  (`self.K2_AttachToActor` _returnvalue self "None" "KeepRelative" "KeepRelative" "KeepRelative" true) ; 생성된 카메라 확인용
  (set `self.CameraActor` _returnvalue))

(event `Wait1Sec`
  ;[1 1 1] 1초 대기
  (`KismetSystemLibrary.Delay` 1.0))

(event `ReturnToPlayer`
  (params (PlayerCharacter :type "Character Object Reference") (PlayerController :type "PlayerController Object Reference"))
  ;[1 1 1] 조사 종료 후 플레이어에게 화면을 자연스럽게 돌린다.
  (`PlayerController.SetViewTargetWithBlend` PlayerController PlayerCharacter 1.0 "VTBlend_Linear" 0.0 false)
  (`PrimitiveComponent.SetCollisionEnabled` (`self.Cube`) "QueryAndPhysics") ; 플레이어에게 카메라가 돌아갈 경우 다시 확대할 수 있으므로 충돌을 재활성
)

(fn `UserConstructionScript`)

(fn `ZoomIn`
  (returns (IsZoomed :type Boolean) (ZoomedActor :type "/Game/BoxesLike/BluePrints/TestBoxBP/BP_CheakPoint Object Reference"))
  ;[1 1 1] 자연스럽게 줌인
  (`PlayerController.SetViewTargetWithBlend` (`GameplayStatics.GetPlayerController` 0) (`self.CameraActor`) 1.0 "VTBlend_Linear" 0.0 false) ; 화면을 뉴 뷰 타겟으로 자연스럽게 이동시키는 명령어\n블랜드 타임이 이동하는 시간
  (`self.Wait1Sec`) ; 함수안에서는 딜레이를 못 씀
  (`PrimitiveComponent.SetCollisionEnabled` (`self.Cube`) "NoCollision") ; 확대중에 스태틱매쉬로 클릭이 안되는 경우가 발생할 수 있으므로 충돌을 삭제
  (return true self))