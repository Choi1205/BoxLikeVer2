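; Block actor that the player rotates in pitch by click-dragging the mouse on it.
; BlockMoving stores the click point and moves input from the Mover to this actor; releasing the left button hands it back.
; While the button is held, mouse axes set MovingMesh's rotation from actor rotation plus a pitch delta.
; The click point's side of the mesh's cached position sets direction: Z for MouseX, X for MouseY.
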(event `self.ReceiveBeginPlay`
  ;[1 1 1] 노드 3개를 계속 끌고다니면 공간을 많이 차지하니 변수화
  (set `self.MyWorldLocation` (`SceneComponent.K2_GetComponentLocation` (`self.MovingMesh`))))

(event `/Game/BoxesLike/BPInterface/BlockMoving.Block Moving`
  (params (Mover :type "Pawn Object Reference") (ClickPoint :type "Vector Structure") (LookingComponentPoint :type "PrimitiveComponent Object Reference"))
  (bind _returnvalue (`GameplayStatics.GetPlayerController` 0))
  ;[1 1 1] 아이템 회전 시작/종료 부분. 클릭하면 플레이어 캐릭터에 있던 컨트롤을 이 액터로 옮긴다.
  (`self.DisableInput` Mover _returnvalue)
  (`self.EnableInput` _returnvalue)
  (set `self.Rotating` true)
  (set `self.MouseLocation` ClickPoint))

(event `Key|LeftMouseButton`
  (params (Key :type "Key Structure"))
  (bind _returnvalue (`GameplayStatics.GetPlayerController` 0))
  ;[1 1 1] 아이템 회전 시작/종료 부분. 클릭하면 플레이어 캐릭터에 있던 컨트롤을 이 액터로 옮긴다.
  (:`Released`
    (`self.DisableInput` _returnvalue)
    (`self.EnableInput` (stale `/Game/BoxesLike/BPInterface/BlockMoving.Block Moving` Mover) _returnvalue)
    (set `self.Rotating` false)))

(event `InputAxisKey|MouseX`
  (params (AxisValue :type "Float (single-precision)"))
  (bind (_myworldlocation_x _myworldlocation_y _myworldlocation_z) (`KismetMathLibrary.BreakVector` (`self.MyWorldLocation`)))
  (bind (_mouselocation_x _mouselocation_y _mouselocation_z) (`KismetMathLibrary.BreakVector` (`self.MouseLocation`)))
  ;[1 1 1] 마우스를 드래그하면 이 스태틱 매쉬가 회전한다. 원하는 축/방향에 맞춰서 X/Y , X/Y/Z 연결 및 Set RotatingDirectionX/Y를 조정
  (if (`PlayerController.IsInputKeyDown` (`GameplayStatics.GetPlayerController` 0) "LeftMouseButton")
    (if (< _myworldlocation_z _mouselocation_z)
      (set `self.RotateDirectionX` 1.0)
      (else
        (set `self.RotateDirectionX` -1.0)))
    (`SceneComponent.K2_SetRelativeRotation` (`self.MovingMesh`) (`KismetMathLibrary.ComposeRotators` (`self.K2_GetActorRotation`) (`KismetMathLibrary.MakeRotator` 0.0 (* AxisValue (`self.RotateDirectionX`)))) false false)))

(event `InputAxisKey|MouseY`
  (params (AxisValue :type "Float (single-precision)"))
  (bind _myworldlocation_x (`KismetMathLibrary.BreakVector` (`self.MyWorldLocation`)))
  (bind _mouselocation_x (`KismetMathLibrary.BreakVector` (`self.MouseLocation`)))
  ;[1 1 1] 마우스를 드래그하면 이 스태틱 매쉬가 회전한다. 원하는 축/방향에 맞춰서 X/Y , X/Y/Z 연결 및 Set RotatingDirectionX/Y를 조정
  (if (`PlayerController.IsInputKeyDown` (`GameplayStatics.GetPlayerController` 0) "LeftMouseButton")
    (if (< _myworldlocation_x _mouselocation_x)
      (set `self.RotateDirectionY` 1.0)
      (else
        (set `self.RotateDirectionY` -1.0)))
    (`SceneComponent.K2_SetRelativeRotation` (`self.MovingMesh`) (`KismetMathLibrary.ComposeRotators` (`self.K2_GetActorRotation`) (`KismetMathLibrary.MakeRotator` 0.0 (* AxisValue (`self.RotateDirectionY`)))) false false)))

(fn `UserConstructionScript`)