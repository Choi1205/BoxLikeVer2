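; BP_ArrayControlSystem is a button-driven actor that cycles red, green and blue laser effects across three Niagara components.
; On BeginPlay it assigns the three laser systems and stores the components in NiagaraData.
; Clicking LeftButton rotates NumData one step left with two swaps.
; Each value then selects the laser asset for the component at the same index, replacing it through SetAsset.
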(event `self.ReceiveBeginPlay`
  (bind _niagaradata (`self.NiagaraData`))
  (bind _niagara_0_ (`self.Niagara[0]`))
  (bind _niagara_1_ (`self.Niagara[1]`))
  (bind _niagara_2_ (`self.Niagara[2]`))
  (`NiagaraComponent.SetAsset` _niagara_0_ "/Game/BoxesLike/VFX/VFS_LaserR.VFS_LaserR" true)
  (`NiagaraComponent.SetAsset` _niagara_1_ "/Game/BoxesLike/VFX/VFS_LaserG.VFS_LaserG" true)
  (`NiagaraComponent.SetAsset` _niagara_2_ "/Game/BoxesLike/VFX/VFS_LaserB.VFS_LaserB" true)
  (`KismetArrayLibrary.Array_Set` _niagaradata 0 _niagara_0_)
  (`KismetArrayLibrary.Array_Set` _niagaradata 1 _niagara_1_)
  (`KismetArrayLibrary.Array_Set` _niagaradata 2 _niagara_2_))

(event `self.LeftButton.OnClicked`
  (params (TouchedComponent :type "PrimitiveComponent Object Reference") (ButtonPressed :type "Key Structure"))
  (bind _numdata (`self.NumData`))
  (`KismetArrayLibrary.Array_Swap` _numdata 0 1)
  (`KismetArrayLibrary.Array_Swap` _numdata 1 2)
  (for (_array_element _array_index) _numdata
    (switch `int` _array_element
      (:`1`
        (bind _output (`|GetArrayItem` (`self.NiagaraData`) _array_index))
        (`NiagaraComponent.SetAsset` _output "/Game/BoxesLike/VFX/VFS_LaserR.VFS_LaserR" true))
      (:`2`
        (`NiagaraComponent.SetAsset` _output "/Game/BoxesLike/VFX/VFS_LaserG.VFS_LaserG" true))
      (:`3`
        (`NiagaraComponent.SetAsset` _output "/Game/BoxesLike/VFX/VFS_LaserB.VFS_LaserB" true)))))

(fn `UserConstructionScript`)