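; Draggable puzzle block actor that slides its MovingMesh along local X with horizontal mouse movement while the left button is held, within a fixed range.
; BlockMoving enables input on the block, and a left-click press disables it and re-enables input on Mover.
; Nearing the positive limit calls Start once on the ClickAndMove actor found at BeginPlay.
; Rotation and Y-axis variants are present but never run.
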(event `self.ReceiveBeginPlay`
  (bind _outactors (`GameplayStatics.GetAllActorsOfClass` "/Game/BoxesLike/BluePrints/TestBoxBP/ClickAndMove.ClickAndMove_C"))
  (set `self.CM_Var` (`|GetArrayItem` _outactors)))

(event `/Game/BoxesLike/BPInterface/BlockMoving.Block Moving`
  (params (Mover :type "Pawn Object Reference") (ClickPoint :type "Vector Structure") (LookingComponentPoint :type "PrimitiveComponent Object Reference"))
  (bind _returnvalue (`GameplayStatics.GetPlayerController` 0))
  ;[1 1 1] 아이템 상세 확인 시작/종료 부분. 상세 확인을 시작하면 플레이어 캐릭터에 있던 컨트롤을 생성된 이 액터로 옮긴다.
  (`self.DisableInput` _returnvalue)
  (`self.EnableInput` _returnvalue))

(event `Key|LeftMouseButton`
  (params (Key :type "Key Structure"))
  (bind _returnvalue (`GameplayStatics.GetPlayerController` 0))
  ;[1 1 1] 아이템 상세 확인 시작/종료 부분. 상세 확인을 시작하면 플레이어 캐릭터에 있던 컨트롤을 생성된 이 액터로 옮긴다.
  (:`Pressed`
    (`self.DisableInput` _returnvalue)
    (`self.EnableInput` (stale `/Game/BoxesLike/BPInterface/BlockMoving.Block Moving` Mover) _returnvalue)))

(event `InputAxisKey|MouseX`
  (params (AxisValue :type "Float (single-precision)"))
  (bind (_relativelocation_x _relativelocation_y _relativelocation_z) (`KismetMathLibrary.BreakVector` (`SceneComponent.RelativeLocation` (`self.MovingMesh`))))
  (bind _relativelocation_x_2 (`KismetMathLibrary.BreakVector` (`SceneComponent.RelativeLocation` (`self.MovingMesh`))))
  (bind _returnvalue (+ _relativelocation_x (* AxisValue -1.0)))
  ;[1 1 1] 마우스를 드래그하면 이 스태틱 매쉬가 이동한다. 원하는 축/방향에 맞춰서 X/Y , XYZ 연결을 조정
  (if (`PlayerController.IsInputKeyDown` (`GameplayStatics.GetPlayerController` 0) "LeftMouseButton")
    (if (and (<= _returnvalue 100.0) (>= _returnvalue -100.0))
      (`SceneComponent.K2_SetRelativeLocation` (`self.MovingMesh`) (`KismetMathLibrary.MakeVector` _returnvalue _relativelocation_y _relativelocation_z) false false)
      (if (and (>= _relativelocation_x_2 99.0) (`self.NotArrive`))
        (`/Game/BoxesLike/BluePrints/TestBoxBP/ClickAndMove.Start` (`self.CM_Var`))
        (set `self.NotArrive` false)))))

(event `InputAxisKey|MouseY`
  (params (AxisValue :type "Float (single-precision)"))
  ;[1 1 1] 마우스를 드래그하면 이 스태틱 매쉬가 이동한다. 원하는 축/방향에 맞춰서 X/Y , XYZ 연결을 조정
)

(fn `UserConstructionScript`)