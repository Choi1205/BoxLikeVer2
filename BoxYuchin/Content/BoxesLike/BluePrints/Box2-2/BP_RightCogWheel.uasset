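; Cogwheel puzzle actor in Box2-2 that the player starts with a key once the preceding spark-point puzzle opens its cover.
; Tick polls that puzzle and the key's item-use point, enabling the point, then sliding in the key mesh.
; Clicking the key hands input to this actor for drag-to-turn.
; Past the roll threshold, control returns and a timeline spins up counter-rotating cogs before RotatingMovement takes over and KeyUsed is set.
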(event `self.ReceiveBeginPlay`
  (`|ExecutionSequence`
    (:`then_0`
      ;[1 1 1] 아이템 사용 포인트 변수로 저장
      (bind _outactors (`GameplayStatics.GetAllActorsWithInterface` "/Game/BoxesLike/BPInterface/ItemUsingPoint.ItemUsingPoint_C"))
      (for _array_element _outactors
        (bind _asbp_item_using_point (cast `/Game/BoxesLike/BluePrints/TestBoxBP/BP_ItemUsingPoint` _array_element))
        (if (== (`/Game/BoxesLike/BluePrints/TestBoxBP/BP_ItemUsingPoint.NeedItemID` _asbp_item_using_point) 26)
          (set `self.Key` _array_element)
          (`PrimitiveComponent.SetCollisionEnabled` (`/Game/BoxesLike/BluePrints/TestBoxBP/BP_ItemUsingPoint.Box` _asbp_item_using_point) "NoCollision"))))
    (:`then_1`
      ;[1 1 1] 이전 퍼즐(레버 당기기) 변수로 저장
      (bind _outactors_2 (`GameplayStatics.GetAllActorsOfClass` "/Game/BoxesLike/BluePrints/Box2-2/BP_SparkPoint.BP_SparkPoint_C"))
      (set `self.SparkPoint` (`|GetArrayItem` _outactors_2)))
    (:`then_2`
      (`MovementComponent.SetUpdatedComponent` (`self.RotatingMovement`) (`self.SM_CogwheelFilled`)))))

(event `self.ReceiveTick`
  (params (DeltaSeconds :type "Float (single-precision)"))
  (bind _key (`self.Key`))
  (bind _keymesh (`self.KeyMesh`))
  (bind _key_2 (`self.Key`))
  (bind (_returnvalue_x _returnvalue_y _returnvalue_z) (`KismetMathLibrary.BreakVector` (`self.K2_GetActorLocation` _key)))
  (bind _relativerotation_roll (`KismetMathLibrary.BreakRotator` (`SceneComponent.RelativeRotation` (`self.KeyMesh`))))
  (`|ExecutionSequence`
    (:`then_0`
      ;[1 1 1] 전극커버가 부착되면 열쇠가 사용가능하게 됨
      (if (`/Game/BoxesLike/BluePrints/Box2-2/BP_SparkPoint.KeyGlassOpen` (`self.SparkPoint`))
        (`/Engine/EditorBlueprintResources/StandardMacros.DoOnce` false
          (:`Completed`
            (`self.K2_SetActorLocation` _key (`KismetMathLibrary.MakeVector` _returnvalue_x (+ _returnvalue_y 5.0) _returnvalue_z) false false)
            (bind _asbp_item_using_point (cast `/Game/BoxesLike/BluePrints/TestBoxBP/BP_ItemUsingPoint` (`self.Key`)))
            (`PrimitiveComponent.SetCollisionEnabled` (`/Game/BoxesLike/BluePrints/TestBoxBP/BP_ItemUsingPoint.Box` _asbp_item_using_point) "QueryAndPhysics")))))
    (:`then_1`
      ;[1 1 1] 열쇠를 사용하고난 뒤 열쇠 사용연출 및 톱니바퀴 회전 시작 연출
      (`/Engine/EditorBlueprintResources/StandardMacros.IsValid` _key_2
        (:`Is Valid`
          (bind _asbp_item_using_point_2 (cast `/Game/BoxesLike/BluePrints/TestBoxBP/BP_ItemUsingPoint` _key_2))
          (if (`/Game/BoxesLike/BluePrints/TestBoxBP/BP_ItemUsingPoint.ItUsed` _asbp_item_using_point_2)
            (`self.K2_DestroyActor` _key_2)))
        (:`Is Not Valid`
          (`/Engine/EditorBlueprintResources/StandardMacros.DoOnce` false
            (:`Completed`
              (`self.DisableInput` (`GameplayStatics.GetPlayerPawn` 0) (`GameplayStatics.GetPlayerController` 0))
              (`StaticMeshComponent.SetStaticMesh` _keymesh "/Game/BoxesLike/Assets/Key/Antique_Key.Antique_Key")
              (set `self.KeyStartLocation` (`SceneComponent.RelativeLocation` _keymesh))
              (set `self.KeyWorldLocation` (`SceneComponent.K2_GetComponentLocation` _keymesh))
              (bind (_direction _value) (`Timeline|KeyMove`)
                (:`Update`
                  (`SceneComponent.K2_SetRelativeLocation` (`self.KeyMesh`) (`KismetMathLibrary.MakeVector` (* _value 60.0)) false false))
                (:`Finished`
                  (`self.EnableInput` (`GameplayStatics.GetPlayerPawn` 0) (`GameplayStatics.GetPlayerController` 0)))))))))
    (:`then_2`
      ;[1 1 1] 좌우 톱니바퀴는 반대로 돌아야함
      (`SceneComponent.K2_SetRelativeRotation` (`self.SM_CogwheelLeft`) (* (`SceneComponent.RelativeRotation` (`self.SM_CogwheelFilled`)) -1.0) false false)
      (`SceneComponent.K2_SetRelativeRotation` (`self.SM_CogwheelRight`) (* (`SceneComponent.RelativeRotation` (`self.SM_CogwheelFilled`)) -1.0) false false))
    (:`then_3`
      (if (< _relativerotation_roll 0.0)
        (`/Engine/EditorBlueprintResources/StandardMacros.DoOnce` false
          (:`Completed`
            (`self.KeyRotatingEnd`)
            (`self.DisableInput` (`GameplayStatics.GetPlayerPawn` 0) (`GameplayStatics.GetPlayerController` 0))
            (`KismetSystemLibrary.Delay` 0.5)
            (`StaticMeshComponent.SetStaticMesh` (`self.KeyMesh`) null)
            (bind (_direction_2 _value_2) (`Timeline|Timeline`) ; 자연스럽게 최고속도로
              (:`Update`
                (`SceneComponent.K2_SetRelativeRotation` (`self.SM_CogwheelFilled`) (`KismetMathLibrary.MakeRotator` 0.0 (* _value_2 240.0)) false false)
                (`SceneComponent.K2_SetRelativeRotation` (`self.SM_CogwheelLeft`) (`KismetMathLibrary.MakeRotator` 0.0 (* _value_2 -240.0)) false false)
                (`SceneComponent.K2_SetRelativeRotation` (`self.SM_CogwheelRight`) (`KismetMathLibrary.MakeRotator` 0.0 (* _value_2 -240.0)) false false))
              (:`Finished`
                (`ActorComponent.Activate` (`self.RotatingMovement`) false)
                (set `self.KeyUsed` true)
                (`self.EnableInput` (`GameplayStatics.GetPlayerPawn` 0) (`GameplayStatics.GetPlayerController` 0))))))))))

(event `/Game/BoxesLike/BPInterface/BlockMoving.Block Moving`
  (params (Mover :type "Pawn Object Reference") (ClickPoint :type "Vector Structure") (LookingComponentPoint :type "PrimitiveComponent Object Reference"))
  (bind _returnvalue (`GameplayStatics.GetPlayerController` 0))
  ;[1 1 1] 아이템 회전 시작/종료 부분. 키를 클릭하면 플레이어 캐릭터에 있던 컨트롤을 이 액터로 옮긴다. 클릭 위치에 따라 회전 방향이 다르다
  (if (== LookingComponentPoint (`self.KeyMesh`))
    (`self.DisableInput` Mover _returnvalue)
    (`self.EnableInput` _returnvalue)
    (set `self.Rotating` true)
    (set `self.MouseLocation` ClickPoint)))

(event `Key|LeftMouseButton`
  (params (Key :type "Key Structure"))
  (bind _returnvalue (`GameplayStatics.GetPlayerController` 0))
  ;[1 1 1] 아이템 회전 시작/종료 부분. 키를 클릭하면 플레이어 캐릭터에 있던 컨트롤을 이 액터로 옮긴다. 클릭 위치에 따라 회전 방향이 다르다
  (:`Released`
    (`self.DisableInput` _returnvalue :!label _label)
    (`self.EnableInput` (stale `/Game/BoxesLike/BPInterface/BlockMoving.Block Moving` Mover) _returnvalue)
    (set `self.Rotating` false)))

(event `KeyRotatingEnd`
  ;[1 1 1] 아이템 회전 시작/종료 부분. 키를 클릭하면 플레이어 캐릭터에 있던 컨트롤을 이 액터로 옮긴다. 클릭 위치에 따라 회전 방향이 다르다
  (goto _label))

(event `InputAxisKey|MouseX`
  (params (AxisValue :type "Float (single-precision)"))
  (bind (_keyworldlocation_x _keyworldlocation_y _keyworldlocation_z) (`KismetMathLibrary.BreakVector` (`self.KeyWorldLocation`)))
  (bind (_mouselocation_x _mouselocation_y _mouselocation_z) (`KismetMathLibrary.BreakVector` (`self.MouseLocation`)))
  ;[1 1 1] 마우스를 드래그하면 키가 회전한다. 원하는 축/방향에 맞춰서 X/Y , X/Y/Z 연결 및 Set RotatingDirectionX/Y를 조정
  (if (`PlayerController.IsInputKeyDown` (`GameplayStatics.GetPlayerController` 0) "LeftMouseButton")
    (if (< _keyworldlocation_z _mouselocation_z)
      (set `self.RotateDirectionX` 1.0)
      (else
        (set `self.RotateDirectionX` -1.0)))
    (`SceneComponent.K2_AddRelativeRotation` (`self.KeyMesh`) (`KismetMathLibrary.ComposeRotators` (`self.K2_GetActorRotation`) (`KismetMathLibrary.MakeRotator` (* AxisValue (`self.RotateDirectionX`)))) false false)))

(event `InputAxisKey|MouseY`
  (params (AxisValue :type "Float (single-precision)"))
  (bind _keyworldlocation_x (`KismetMathLibrary.BreakVector` (`self.KeyWorldLocation`)))
  (bind _mouselocation_x (`KismetMathLibrary.BreakVector` (`self.MouseLocation`)))
  ;[1 1 1] 마우스를 드래그하면 키가 회전한다. 원하는 축/방향에 맞춰서 X/Y , X/Y/Z 연결 및 Set RotatingDirectionX/Y를 조정
  (if (`PlayerController.IsInputKeyDown` (`GameplayStatics.GetPlayerController` 0) "LeftMouseButton")
    (if (< _keyworldlocation_x _mouselocation_x)
      (set `self.RotateDirectionY` 1.0)
      (else
        (set `self.RotateDirectionY` -1.0)))
    (`SceneComponent.K2_AddRelativeRotation` (`self.KeyMesh`) (`KismetMathLibrary.ComposeRotators` (`self.K2_GetActorRotation`) (`KismetMathLibrary.MakeRotator` (* AxisValue (`self.RotateDirectionY`)))) false false)))

(fn `UserConstructionScript`)