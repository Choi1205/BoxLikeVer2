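; BP_DrainCover is a clickable drain cover that swings open once to reveal a hidden battery item.
; On BeginPlay it finds the BP_ItemActor with the battery's ItemID and clears its mesh.
; The first click restores the battery mesh, then chains two timelines: one rotates the cover open, the next raises the battery.
; Player input is disabled throughout the sequence so the battery cannot be picked up mid-animation.
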(event `self.ReceiveBeginPlay`
  ;[1 1 1] 커버 아래의 배터리를 찾아서 연결함. 아이템은 모두 ItemActor BP이므로 ID값을 이용하여 찾는다.
  (bind _outactors (`GameplayStatics.GetAllActorsOfClass` "/Game/BoxesLike/BluePrints/TestBoxBP/BP_ItemActor.BP_ItemActor_C"))
  (for _array_element _outactors
    (if (== (`/Game/BoxesLike/BluePrints/TestBoxBP/BP_ItemActor.ItemID` _array_element) 23)
      (bind _output_get (set `self.Battery` _array_element))
      (`StaticMeshComponent.SetStaticMesh` (`/Game/BoxesLike/BluePrints/TestBoxBP/BP_ItemActor.StaticMesh` _output_get) null))))

(event `self.S_Metal_Drain_Cover.OnClicked`
  (params (TouchedComponent :type "PrimitiveComponent Object Reference") (ButtonPressed :type "Key Structure"))
  (bind (_returnvalue_x _returnvalue_y _returnvalue_z) (`KismetMathLibrary.BreakVector` (`self.K2_GetActorLocation` (`self.Battery`))))
  ;[1 1 1] 커버를 클릭하면 커버가 열리고 배터리가 튀어나온다. 배터리가 나오는 도중 집어갈 수 없도록 나오는동안 입력을 차단한다.
  (`/Engine/EditorBlueprintResources/StandardMacros.DoOnce` false
    (:`Completed`
      (`self.DisableInput` (`GameplayStatics.GetPlayerPawn` 0) (`GameplayStatics.GetPlayerController` 0))
      (`StaticMeshComponent.SetStaticMesh` (`/Game/BoxesLike/BluePrints/TestBoxBP/BP_ItemActor.StaticMesh` (`self.Battery`)) "/Game/BoxesLike/Assets/9VBattery/9V_Battery.9V_Battery")
      (bind (_direction _coveropen) (`Timeline|OpenCover`) ; 커버가 열려요
        (:`Update`
          (`SceneComponent.K2_SetRelativeRotation` (`self.S_Metal_Drain_Cover`) (`KismetMathLibrary.MakeRotator` (* _coveropen 80.0) 0.0 90.0) false false))
        (:`Finished`
          (set `self.BatteryStartZ` _returnvalue_z)
          (bind (_direction_2 _rise) (`Timeline|BatteryRise`) ; 배터리가 튀어나와요
            (:`Update`
              (`self.K2_SetActorLocation` (`self.Battery`) (`KismetMathLibrary.MakeVector` _returnvalue_x _returnvalue_y (+ (* _rise 10.0) (`self.BatteryStartZ`))) false false))
            (:`Finished`
              (`self.EnableInput` (`GameplayStatics.GetPlayerPawn` 0) (`GameplayStatics.GetPlayerController` 0)))))))))

(fn `UserConstructionScript`)