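; Rear-table puzzle switch: clicking it presses the button and extends two electrode pins, then raises a push lever if FlipComplete is set.
; Otherwise nested FlipFlops and an IsA flag reverse the pin and button timelines, restoring input afterward.
; BeginPlay finds the lever by ItemID and clears its mesh until the reveal, which blocks further clicks.
; Button and pins move by timeline-driven relative offsets scaled by Tick's DeltaSeconds.
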(event `self.ReceiveTick`
  (params (DeltaSeconds :type "Float (single-precision)"))
  ;[1 1 1] 여기저기서 써서 변수화
  (set `self.Delta Seconds` DeltaSeconds))

(event `self.ReceiveBeginPlay`
  ;[1 1 1] 레버를 찾아서 변수에 저장
  (bind _outactors (`GameplayStatics.GetAllActorsOfClass` "/Game/BoxesLike/BluePrints/TestBoxBP/BP_ItemActor.BP_ItemActor_C"))
  (for _array_element _outactors
    (if (== (`/Game/BoxesLike/BluePrints/TestBoxBP/BP_ItemActor.ItemID` _array_element) 25)
      (bind _output_get (set `self.PushLever` _array_element))
      (`StaticMeshComponent.SetStaticMesh` (`/Game/BoxesLike/BluePrints/TestBoxBP/BP_ItemActor.StaticMesh` _output_get) null))))

(event `self.SwitchButton.OnClicked`
  (params (TouchedComponent :type "PrimitiveComponent Object Reference") (ButtonPressed :type "Key Structure"))
  (bind (_returnvalue_x _returnvalue_y _returnvalue_z) (`KismetMathLibrary.BreakVector` (`self.K2_GetActorLocation` (`self.PushLever`))))
  ;[1 1 1] 버튼 눌림, 전극 나옴, 레버 올라옴 애니메이션 구간.
  (if (not (`self.GetLever`))
    (`/Engine/EditorBlueprintResources/StandardMacros.FlipFlop` :!label _label
      (:`A`
        (`self.DisableInput` (`GameplayStatics.GetPlayerPawn` 0) (`GameplayStatics.GetPlayerController` 0))
        (bind (_direction _value) (`Timeline|SwitchMove` :!via `PlayFromStart` :!label _label_2) ; A : 버튼이 눌림, B : 버튼이 튀어나옴
          (:`Update`
            (`SceneComponent.K2_AddRelativeLocation` (`self.SwitchButton`) (`KismetMathLibrary.MakeVector` 0.0 0.0 (* _value (`self.SwitchMovement`) (`self.Delta Seconds`))) false false) ; set로하면 동작이 이상해서 만들어 둔 Add를 썼다.
          )
          (:`Finished`
            (`/Engine/EditorBlueprintResources/StandardMacros.FlipFlop`
              (:`A`
                (bind (_direction_2 _value_2) (`Timeline|PinMove` :!via `PlayFromStart` :!label _label_3) ; A : 전극이 튀어나옴, B : 전극이 들어감
                  (:`Update`
                    (`SceneComponent.K2_AddRelativeLocation` (`self.ElecPinR`) (`KismetMathLibrary.MakeVector` (* _value_2 (`self.PinMovement`) (`self.Delta Seconds`))) false false)
                    (`SceneComponent.K2_AddRelativeLocation` (`self.ElecPinL`) (`KismetMathLibrary.MakeVector` (* _value_2 (`self.PinMovement`) (`self.Delta Seconds`))) false false))
                  (:`Finished`
                    (if (`self.IsA`)
                      (if (`self.FlipComplete`)
                        (set `self.LeverStartZ` _returnvalue_z) ; 이쪽으로 빠지면 플립플롭 B는 실행되지 않음
                        (`StaticMeshComponent.SetStaticMesh` (`/Game/BoxesLike/BluePrints/TestBoxBP/BP_ItemActor.StaticMesh` (`self.PushLever`)) "/Game/BoxesLike/StaticMesh/Box2-2/SM_PushLever.SM_PushLever")
                        (bind (_direction_3 _rise) (`Timeline|LeverUP`)
                          (:`Update`
                            (`self.K2_SetActorLocation` (`self.PushLever`) (`KismetMathLibrary.MakeVector` _returnvalue_x _returnvalue_y (+ (* _rise 10.0) (`self.LeverStartZ`))) false false)
                            (set `self.GetLever` true))
                          (:`Finished`
                            (`self.EnableInput` (`GameplayStatics.GetPlayerPawn` 0) (`GameplayStatics.GetPlayerController` 0))))
                        (else
                          (set `self.IsA` false)
                          (set `self.SwitchMovement` 3.5)
                          (set `self.PinMovement` -8.0)
                          (goto _label)))
                      (else
                        (goto _label_2 :!via `ReverseFromEnd`))))))
              (:`B`
                (set `self.SwitchMovement` -3.5)
                (set `self.PinMovement` 8.0)
                (set `self.IsA` true)
                (`self.EnableInput` (`GameplayStatics.GetPlayerPawn` 0) (`GameplayStatics.GetPlayerController` 0)))))))
      (:`B`
        (goto _label_3 :!via `ReverseFromEnd`)))))

(fn `UserConstructionScript`)