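; Puzzle-box front cover that unlocks when its bolt is unscrewed, then slides open by mouse drag.
; BeginPlay finds the bolt's use point and hides the key item's mesh.
; Tick destroys the used point, then runs one timeline forward and reversed to insert and withdraw a spinning screwdriver with the bolt, restoring the key mesh.
; BlockMoving then takes input from the Mover until mouse release, allowing clamped one-way X sliding.
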(event `self.ReceiveBeginPlay`
  ;[1 1 1] 아이템 사용 포인트 변수로 저장
  (`|ExecutionSequence`
    (:`then_0`
      (bind _outactors (`GameplayStatics.GetAllActorsWithInterface` "/Game/BoxesLike/BPInterface/ItemUsingPoint.ItemUsingPoint_C"))
      (for _array_element _outactors
        (bind _asbp_item_using_point (cast `/Game/BoxesLike/BluePrints/TestBoxBP/BP_ItemUsingPoint` _array_element))
        (if (== (`/Game/BoxesLike/BluePrints/TestBoxBP/BP_ItemUsingPoint.NeedItemID` _asbp_item_using_point) 24)
          (set `self.Bolt` _array_element))))
    (:`then_1`
      (bind _outactors_2 (`GameplayStatics.GetAllActorsOfClass` "/Game/BoxesLike/BluePrints/TestBoxBP/BP_ItemActor.BP_ItemActor_C"))
      (for _array_element_2 _outactors_2
        (if (== (`/Game/BoxesLike/BluePrints/TestBoxBP/BP_ItemActor.ItemID` _array_element_2) 26)
          (bind _output_get (set `self.Key` _array_element_2))
          (`StaticMeshComponent.SetStaticMesh` (`/Game/BoxesLike/BluePrints/TestBoxBP/BP_ItemActor.StaticMesh` _output_get) null))))
    (:`then_2`
      (`MovementComponent.SetUpdatedComponent` (`self.RotatingMovement`) (`self.Driver`)) ; RotatingMovement가 드라이버만 돌리도록 설정
    )))

(event `/Game/BoxesLike/BPInterface/BlockMoving.Block Moving`
  (params (Mover :type "Pawn Object Reference") (ClickPoint :type "Vector Structure") (LookingComponentPoint :type "PrimitiveComponent Object Reference"))
  (bind _returnvalue (`GameplayStatics.GetPlayerController` 0))
  ;[1 1 1] 아이템 상세 확인 시작/종료 부분. 상세 확인을 시작하면 플레이어 캐릭터에 있던 컨트롤을 생성된 이 액터로 옮긴다.
  (if (`self.BoltUsed`)
    (`self.DisableInput` Mover _returnvalue)
    (`self.EnableInput` _returnvalue)))

(event `Key|LeftMouseButton`
  (params (Key :type "Key Structure"))
  (bind _returnvalue (`GameplayStatics.GetPlayerController` 0))
  ;[1 1 1] 아이템 상세 확인 시작/종료 부분. 상세 확인을 시작하면 플레이어 캐릭터에 있던 컨트롤을 생성된 이 액터로 옮긴다.
  (:`Released`
    (`self.DisableInput` _returnvalue)
    (`self.EnableInput` (stale `/Game/BoxesLike/BPInterface/BlockMoving.Block Moving` Mover) _returnvalue)))

(event `self.ReceiveTick`
  (params (DeltaSeconds :type "Float (single-precision)"))
  (bind _driver (`self.Driver`))
  (bind _driver_2 (`self.Driver`))
  (bind _bolt (`self.Bolt`))
  (bind (_relativelocation_x _relativelocation_y _relativelocation_z) (`KismetMathLibrary.BreakVector` (`SceneComponent.RelativeLocation` (`self.SM_GunBoxRearButton`))))
  (bind _relativerotation_roll (`KismetMathLibrary.BreakRotator` (`SceneComponent.RelativeRotation` (`self.Driver`))))
  (`|ExecutionSequence`
    (:`then_0`
      ;[1 1 1] 드라이버 사용시 실행. NotVaild이후는 드라이버, 볼트 이동 애니메이션
      (`/Engine/EditorBlueprintResources/StandardMacros.IsValid` _bolt
        (:`Is Valid`
          (bind _asbp_item_using_point (cast `/Game/BoxesLike/BluePrints/TestBoxBP/BP_ItemUsingPoint` _bolt))
          (if (`/Game/BoxesLike/BluePrints/TestBoxBP/BP_ItemUsingPoint.ItUsed` _asbp_item_using_point)
            (`self.K2_DestroyActor` _bolt)))
        (:`Is Not Valid`
          ;[1 1 1] 드라이버를 꽃고, 볼트를 풀어 빼내는 연출
          (`/Engine/EditorBlueprintResources/StandardMacros.DoOnce` false
            (:`Completed`
              (`StaticMeshComponent.SetStaticMesh` _driver_2 "/Game/BoxesLike/StaticMesh/Box2-2/SM_ScrewDriver.SM_ScrewDriver")
              (bind (_direction _value) (`Timeline|DriverMove` :!via `PlayFromStart` :!label _label) ; A : 드라이버를 꽃아요. B 드라이버가 돌아가며 빠져요
                (:`Update`
                  (`SceneComponent.K2_SetRelativeLocation` _driver_2 (`KismetMathLibrary.MakeVector` (* _value 3.0)) false false) ; 드라이버는 A,B 모두 움직여요
                  (if (`self.IsB`)
                    (`SceneComponent.K2_SetRelativeLocation` (`self.SM_GunBoxRearButton`) (`KismetMathLibrary.MakeVector` -7.0 0.0 (+ (* (- 1.0 _value) 1.25) (`self.BoltStartLocation`))) false false)))
                (:`Finished`
                  (`/Engine/EditorBlueprintResources/StandardMacros.FlipFlop`
                    (:`A`
                      (`KismetSystemLibrary.Delay` 0.5) ; 빠지기전 잠깐 멈추고
                      (`ActorComponent.Activate` (`self.RotatingMovement`) false)
                      (set `self.BoltStartLocation` _relativelocation_z)
                      (set `self.IsB` true)
                      (goto _label :!via `ReverseFromEnd`))
                    (:`B`
                      (`StaticMeshComponent.SetStaticMesh` _driver null)
                      (`ActorComponent.Deactivate` (`self.RotatingMovement`))
                      (`ActorComponent.K2_DestroyComponent` _driver)
                      (`ActorComponent.K2_DestroyComponent` (`self.RotatingMovement`))
                      (`ActorComponent.K2_DestroyComponent` (`self.SM_GunBoxRearButton`))
                      (`ActorComponent.K2_DestroyComponent` (`self.DriverPoint`))
                      (set `self.BoltUsed` true)
                      (`StaticMeshComponent.SetStaticMesh` (`/Game/BoxesLike/BluePrints/TestBoxBP/BP_ItemActor.StaticMesh` (`self.Key`)) "/Game/BoxesLike/Assets/Key/Antique_Key.Antique_Key"))))))))))
    (:`then_1`
      ;[1 1 1] 드라이버를 사용애니메이션 중 드라이버가 빠질 때 볼트도 같이 회전하면서 빠져나온다
      (`/Engine/EditorBlueprintResources/StandardMacros.IsValid` (`self.SM_GunBoxRearButton`)
        (:`Is Valid`
          (if (`self.IsB`)
            (`SceneComponent.K2_SetRelativeRotation` (`self.SM_GunBoxRearButton`) (`KismetMathLibrary.MakeRotator` 0.0 0.0 (* _relativerotation_roll -0.5)) false false)))))))

(event `InputAxisKey|MouseX`
  (params (AxisValue :type "Float (single-precision)"))
  (bind _relativelocation_x (`KismetMathLibrary.BreakVector` (`SceneComponent.RelativeLocation` (`self.SM_FrontCover`))))
  (bind (_relativelocation_x_2 _relativelocation_y _relativelocation_z) (`KismetMathLibrary.BreakVector` (`SceneComponent.RelativeLocation` (`self.SM_FrontCover`))))
  (bind _returnvalue (+ (* AxisValue 0.5) _relativelocation_x_2))
  ;[1 1 1] 마우스를 드래그하면 이 스태틱 매쉬가 이동한다. 원하는 축/방향에 맞춰서 X/Y , XYZ 연결을 조정.
  (if (and (> AxisValue 0.0) (< _relativelocation_x 16.0) (`PlayerController.IsInputKeyDown` (`GameplayStatics.GetPlayerController` 0) "LeftMouseButton"))
    (`SceneComponent.K2_SetRelativeLocation` (`self.SM_FrontCover`) (`KismetMathLibrary.MakeVector` _returnvalue _relativelocation_y _relativelocation_z) false false)
    (if (> _returnvalue 16.0)
      (`SceneComponent.K2_SetRelativeLocation` (`self.SM_FrontCover`) (`KismetMathLibrary.MakeVector` 16.0 _relativelocation_y _relativelocation_z) false false))))

(fn `UserConstructionScript`)