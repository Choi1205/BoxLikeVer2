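; BP_Moving2WaySample is a sample draggable block actor whose mesh slides along one of two axes.
; BlockMoving shifts input from the Mover to this actor; the logic handing it back is unwired.
; While left mouse is held, inverted MouseX moves MovingMesh on relative X or Y, chosen by comparing ClickPoint.X with the mesh's world X, without sweep.
; MouseY is an empty event.
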(event `/Game/BoxesLike/BPInterface/BlockMoving.Block Moving`
  (params (Mover :type "Pawn Object Reference") (ClickPoint :type "Vector Structure") (LookingComponentPoint :type "PrimitiveComponent Object Reference"))
  (bind _returnvalue (`GameplayStatics.GetPlayerController` 0))
  ;[1 1 1] 아이템 상세 확인 시작/종료 부분. 상세 확인을 시작하면 플레이어 캐릭터에 있던 컨트롤을 생성된 이 액터로 옮긴다.
  (`self.DisableInput` Mover _returnvalue)
  (`self.EnableInput` _returnvalue))

(event `Key|LeftMouseButton`
  (params (Key :type "Key Structure"))
  ;[1 1 1] 아이템 상세 확인 시작/종료 부분. 상세 확인을 시작하면 플레이어 캐릭터에 있던 컨트롤을 생성된 이 액터로 옮긴다.
)

(event `InputAxisKey|MouseX`
  (params (AxisValue :type "Float (single-precision)"))
  (bind _movingmesh (`self.MovingMesh`))
  (bind _returnvalue_x (`KismetMathLibrary.BreakVector` (`SceneComponent.K2_GetComponentLocation` _movingmesh)))
  (bind (_relativelocation_x _relativelocation_y _relativelocation_z) (`KismetMathLibrary.BreakVector` (`SceneComponent.RelativeLocation` (`self.MovingMesh`))))
  (bind (_relativelocation_x_2 _relativelocation_y_2 _relativelocation_z_2) (`KismetMathLibrary.BreakVector` (`SceneComponent.RelativeLocation` _movingmesh)))
  ;[1 1 1] 마우스를 드래그하면 이 스태틱 매쉬가 이동한다. 원하는 축/방향에 맞춰서 X/Y , XYZ 연결을 조정
  (if (`PlayerController.IsInputKeyDown` (`GameplayStatics.GetPlayerController` 0) "LeftMouseButton")
    (if (> (.x (stale `/Game/BoxesLike/BPInterface/BlockMoving.Block Moving` ClickPoint)) _returnvalue_x)
      (`SceneComponent.K2_SetRelativeLocation` (`self.MovingMesh`) (`KismetMathLibrary.MakeVector` (+ _relativelocation_x_2 (* AxisValue -1.0)) _relativelocation_y_2 _relativelocation_z_2) false false)
      (else
        (`SceneComponent.K2_SetRelativeLocation` (`self.MovingMesh`) (`KismetMathLibrary.MakeVector` _relativelocation_x (+ _relativelocation_y (* (stale `InputAxisKey|MouseY` AxisValue) -1.0)) _relativelocation_z) false false)))))

(event `InputAxisKey|MouseY`
  (params (AxisValue :type "Float (single-precision)"))
  ;[1 1 1] 마우스를 드래그하면 이 스태틱 매쉬가 이동한다. 원하는 축/방향에 맞춰서 X/Y , XYZ 연결을 조정
)

(fn `UserConstructionScript`)