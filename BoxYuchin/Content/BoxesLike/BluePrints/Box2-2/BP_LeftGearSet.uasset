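; Left gear set for the Box2-2 puzzle that starts spinning once the right cogwheel's key is used or its top gear is clicked.
; A one-shot trigger swaps the Niagara effects to light blue and plays a spin-up timeline with alternating gear directions.
; When the timeline finishes, RotatingMovement drives the top gear and SpinStart is set.
; Tick mirrors the top gear's rotation onto the other gears, negated for counter-rotating ones.
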(event `self.ReceiveBeginPlay`
  (bind _outactors (`GameplayStatics.GetAllActorsOfClass` "/Game/BoxesLike/BluePrints/Box2-2/BP_RightCogWheel.BP_RightCogWheel_C"))
  (set `self.RightCogWheel` (`|GetArrayItem` _outactors))
  (`MovementComponent.SetUpdatedComponent` (`self.RotatingMovement`) (`self.StylizedGearTop`)))

(event `self.ReceiveTick`
  (params (DeltaSeconds :type "Float (single-precision)"))
  (bind _relativerotation (`SceneComponent.RelativeRotation` (`self.StylizedGearTop`)))
  (`|ExecutionSequence`
    (:`then_0`
      (if (`/Game/BoxesLike/BluePrints/Box2-2/BP_RightCogWheel.KeyUsed` (`self.RightCogWheel`))
        (`/Engine/EditorBlueprintResources/StandardMacros.DoOnce` false :!label _label
          (:`Completed`
            (`NiagaraComponent.SetAsset` (`self.NiagaraB`) "/Game/BoxesLike/VFX/Box2-2/VFS_GearLightBlue.VFS_GearLightBlue" true)
            (`NiagaraComponent.SetAsset` (`self.NiagaraT`) "/Game/BoxesLike/VFX/Box2-2/VFS_GearLightBlue.VFS_GearLightBlue" true)
            (`NiagaraComponent.SetAsset` (`self.NiagaraTL`) "/Game/BoxesLike/VFX/Box2-2/VFS_GearLightBlue.VFS_GearLightBlue" true)
            (`NiagaraComponent.SetAsset` (`self.NiagaraBR`) "/Game/BoxesLike/VFX/Box2-2/VFS_GearLightBlue.VFS_GearLightBlue" true)
            (bind (_direction _value) (`Timeline|Timeline`)
              (:`Update`
                (`SceneComponent.K2_SetRelativeRotation` (`self.StylizedGearBottomRight`) (`KismetMathLibrary.MakeRotator` (* _value 240.0)) false false)
                (`SceneComponent.K2_SetRelativeRotation` (`self.StylizedGearTop`) (`KismetMathLibrary.MakeRotator` (* _value 240.0)) false false)
                (`SceneComponent.K2_SetRelativeRotation` (`self.StylizedGearBottom`) (`KismetMathLibrary.MakeRotator` (* _value -240.0)) false false)
                (`SceneComponent.K2_SetRelativeRotation` (`self.StylizedGearTopLeft`) (`KismetMathLibrary.MakeRotator` (* _value -240.0)) false false))
              (:`Finished`
                (`ActorComponent.Activate` (`self.RotatingMovement`) false)
                (set `self.SpinStart` true)))))))
    (:`then_1`
      (`SceneComponent.K2_SetRelativeRotation` (`self.StylizedGearBottom`) (* _relativerotation -1.0) false false)
      (`SceneComponent.K2_SetRelativeRotation` (`self.StylizedGearTopLeft`) (* _relativerotation -1.0) false false)
      (`SceneComponent.K2_SetRelativeRotation` (`self.StylizedGearBottomRight`) _relativerotation false false))))

(event `self.StylizedGearTop.OnClicked`
  (params (TouchedComponent :type "PrimitiveComponent Object Reference") (ButtonPressed :type "Key Structure"))
  (goto _label))

(fn `UserConstructionScript`)