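; BP_ClearTable is the game-clear table that shows the final key and power cell being inserted and triggers the ending fade-out.
; BeginPlay finds the two matching BP_ItemUsingPoint actors by their NeedItemID.
; Tick polls each point's ItUsed flag, then once sets that item's mesh and slides it in with a timeline.
; When both animations finish, it calls FadeOut once on the player's inventory widget, where an ending cutscene is still to be added.
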(event `self.ReceiveBeginPlay`
  ;[1 1 1] 게임 시작시 최종 아이템 사용 포인트 BP와 연결
  (bind _outactors (`GameplayStatics.GetAllActorsWithInterface` "/Game/BoxesLike/BPInterface/ItemUsingPoint.ItemUsingPoint_C")) ; 키 & 파워셀 사용포인트 연결
  (for _array_element _outactors
    (bind _asbp_item_using_point (cast `/Game/BoxesLike/BluePrints/TestBoxBP/BP_ItemUsingPoint` _array_element))
    (if (== (`/Game/BoxesLike/BluePrints/TestBoxBP/BP_ItemUsingPoint.NeedItemID` _asbp_item_using_point) 13)
      (set `self.KeyUsingPoint` _array_element)
      (elif (== (`/Game/BoxesLike/BluePrints/TestBoxBP/BP_ItemUsingPoint.NeedItemID` _asbp_item_using_point) 29)
        (set `self.CellUsingPoint` _array_element)))))

(event `self.ReceiveTick`
  (params (DeltaSeconds :type "Float (single-precision)"))
  (bind _key (`self.Key`))
  (bind _cell (`self.Cell`))
  ;[1 1 1] 시퀸스 0,1 : 각 최종 아이템이 사용됬을때 삽입되는 연출. 시퀸스2 : 최종아이템이 모두 사용되면 클리어 화면을 출력함
  (`|ExecutionSequence`
    (:`then_0`
      (bind _asbp_item_using_point (cast `/Game/BoxesLike/BluePrints/TestBoxBP/BP_ItemUsingPoint` (`self.KeyUsingPoint`)))
      (if (`/Game/BoxesLike/BluePrints/TestBoxBP/BP_ItemUsingPoint.ItUsed` _asbp_item_using_point)
        (`/Engine/EditorBlueprintResources/StandardMacros.DoOnce` false
          (:`Completed`
            (`StaticMeshComponent.SetStaticMesh` _key "/Game/BoxesLike/Assets/Key/Antique_Key.Antique_Key")
            (bind (_direction _keyvalue) (`Timeline|KeyMove`)
              (:`Update`
                (`SceneComponent.K2_SetRelativeLocation` _key (`KismetMathLibrary.MakeVector` (* _keyvalue 40.0)) false false))
              (:`Finished`
                (set `self.KeyAnimEnd` true)))))))
    (:`then_1`
      (bind _asbp_item_using_point_2 (cast `/Game/BoxesLike/BluePrints/TestBoxBP/BP_ItemUsingPoint` (`self.CellUsingPoint`)))
      (if (`/Game/BoxesLike/BluePrints/TestBoxBP/BP_ItemUsingPoint.ItUsed` _asbp_item_using_point_2)
        (`/Engine/EditorBlueprintResources/StandardMacros.DoOnce` false
          (:`Completed`
            (`StaticMeshComponent.SetStaticMesh` _cell "/Game/BoxesLike/Assets/PowerCellEc/EC_Power_Cell.EC_Power_Cell")
            (bind (_direction_2 _cellvalue) (`Timeline|CellMove`)
              (:`Update`
                (`SceneComponent.K2_SetRelativeLocation` _cell (`KismetMathLibrary.MakeVector` (* _cellvalue 55.0)) false false))
              (:`Finished`
                (set `self.CellAnimEnd` true)))))))
    (:`then_2`
      (if (and (`self.KeyAnimEnd`) (`self.CellAnimEnd`))
        (`/Engine/EditorBlueprintResources/StandardMacros.DoOnce` false ; 이 뒤쪽에 엔딩 컷신이 들어가야한다
          (:`Completed`
            (bind _asbp_first_person_character (cast `/Game/FirstPerson/Blueprints/BP_FirstPersonCharacter` (`GameplayStatics.GetPlayerCharacter` 0)))
            (`/Game/BoxesLike/BluePrints/UI_OnScreenWidget.FadeOut` (`/Game/FirstPerson/Blueprints/BP_FirstPersonCharacter.InvenWidget` _asbp_first_person_character))))))))

(fn `UserConstructionScript`)